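; BP_GameplayLevelData is a per-level store of tag-keyed bool and int values for gameplay state.
; On BeginPlay it casts the game mode to BP_GameMode_TemplateBase, caches it and registers itself as the level data source.
; Setters write to the maps and notify the game mode of the changed tag.
; TryGet functions return each value with a validity flag.
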(event EventSetLevelInt
  (params (LevelIntTag :type Gameplay%20Tag%20Structure) (NewValue :type Integer))
  (bind _gamemode (Variables|Default|GetGameMode))
  (Utilities|Map|Add (Variables|Default|GetLevelInts) LevelIntTag NewValue)
  (Utilities|IsValid _gamemode
    (:Is%20Valid
      (Default|NotifyLevelIntValueUpdated _gamemode self LevelIntTag))))

(event EventSetLevelBool
  (params (LevelBoolTag :type Gameplay%20Tag%20Structure) (NewValue :type Boolean))
  (bind _gamemode (Variables|Default|GetGameMode))
  (Utilities|Map|Add (Variables|Default|GetLevelBools) LevelBoolTag NewValue)
  (Utilities|IsValid _gamemode
    (:Is%20Valid
      (Default|NotifyLevelBoolValueUpdated _gamemode self LevelBoolTag))))

(event EventBeginPlay
  (bind _asbp_game_mode_template_base (Utilities|Casting|CastToBP_GameMode_TemplateBase (Game|GetGameMode)))
  (bind _output_get (Variables|Default|SetGameMode _asbp_game_mode_template_base))
  (Default|UpdateGameplayLevelDataSource _asbp_game_mode_template_base self))

(fn ConstructionScript)

(fn TryGetLevelBool
  (params (LevelBoolTag :type Gameplay%20Tag%20Structure))
  (bind _levelbools (Variables|Default|GetLevelBools))
  (bind (_value _returnvalue) (Utilities|Map|Find _levelbools LevelBoolTag))
  (return _value _returnvalue))

(fn TryGetLevelInt
  (params (LevelIntTag :type Gameplay%20Tag%20Structure))
  (bind _levelints (Variables|Default|GetLevelInts))
  (bind (_value _returnvalue) (Utilities|Map|Find _levelints LevelIntTag))
  (return _value _returnvalue))