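; Template cheat manager that provides debug commands for slow motion and a debug mode toggle.
; SlomoUp and SlomoDown step global time dilation through the SlomoSettings array, clamped at both ends, and print the result on screen.
; An unmatched current dilation falls back to 1.0 when the array has entries.
; ToggleDebugMode flips a state and sends it to every BPI_Debuggable actor and those actors' BPI_Debuggable components.
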(event Custom|SlomoUp
  (bind (_index _settingfound) (CallFunction|FindCurrentSlomoSettingIndex))
  (if _settingfound
    (CallFunction|UpdateSlomo (Utilities|Array|Get(acopy) (Variables|Default|GetSlomoSettings) (Math|Integer|Min(Integer) (+ _index 1) (- (Utilities|Array|Length (Variables|Default|GetSlomoSettings)) 1))))
    (else
      (CallFunction|SlomoFallback))))

(event Custom|SlomoDown
  (bind (_index _settingfound) (CallFunction|FindCurrentSlomoSettingIndex))
  (if _settingfound
    (CallFunction|UpdateSlomo (Utilities|Array|Get(acopy) (Variables|Default|GetSlomoSettings) (Math|Integer|Max(Integer) (- _index 1))))
    (else
      (CallFunction|SlomoFallback))))

(event Custom|UpdateSlomo
  (params (CurrentSlomo :type Float%20%28double-precision%29))
  (Utilities|Time|SetGlobalTimeDilation CurrentSlomo)
  (Development|PrintString (Utilities|String|Append "Time Dialation: " (Utilities|String|ToString(Float) (Class|GameplayStatics|GetGlobalTimeDilation))) true true "(R=1.000000,G=0.701344,B=0.344081,A=1.000000)" 5.0 "TimeDilation"))

(event Custom|SlomoFallback
  (if (> (Utilities|Array|Length (Variables|Default|GetSlomoSettings)) 0)
    (CallFunction|UpdateSlomo 1.0)
    (else
      (CallFunction|UpdateSlomo (Utilities|Array|Get(acopy) (Variables|Default|GetSlomoSettings) (Math|Float|Floor (* (Math|Conversions|ToFloat(Integer) (Utilities|Array|Length (Variables|Default|GetSlomoSettings))) 0.5)))))))

(event Custom|ToggleDebugMode
  (bind _isa (Utilities|FlowControl|FlipFlop)
    (:A
      _)
    (:B
      _))
  (bind _outactors (Actor|GetAllActorswithInterface "/Game/EpicTemplates/TemplateAgnostic/Blueprints/Interfaces/BPI_Debuggable.BPI_Debuggable_C"))
  (for _array_element _outactors
    (Class|BPIDebuggable|UpdateIsinDebug(Message) _array_element _isa)
    (for _array_element_2 (Class|Actor|GetComponentsbyInterface _array_element "/Game/EpicTemplates/TemplateAgnostic/Blueprints/Interfaces/BPI_Debuggable.BPI_Debuggable_C")
      (Class|BPIDebuggable|UpdateIsinDebug(Message) _array_element_2 _isa))))

(fn FindCurrentSlomoSettingIndex
  (LocalVariables|SetCurrentTimeDilation (Class|GameplayStatics|GetGlobalTimeDilation))
  (for (_array_element _array_index) (Variables|Default|GetSlomoSettings)
    (if (Math|Float|NearlyEqual(Float) _array_element (LocalVariables|GetCurrentTimeDilation) 0.001)
      (return _array_index true)))
  (return -1 false))