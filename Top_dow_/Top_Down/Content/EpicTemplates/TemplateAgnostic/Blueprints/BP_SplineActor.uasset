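; BP_SplineActor is a spline path actor that tracks the actors following it through their BP_SplineFollowerComponent.
; Followers are registered in a map on start and removed when they stop or are destroyed, with event bindings managed along the way.
; It relays start, stop, notify-point and target-reached events through its own dispatchers.
; Query functions expose the spline, its notify points, whether an actor is on it and whether it is in use.
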(event Custom|OnFollowingActorDestroyed
  (params (DestroyedActor :type Actor%20Object%20Reference))
  (CallFunction|CleanupFollower DestroyedActor (Actor|GetComponentbyClass DestroyedActor "/Game/EpicTemplates/TemplateAgnostic/Blueprints/Components/BP_SplineFollowerComponent.BP_SplineFollowerComponent_C")))

(event Custom|FollowerReachedTarget
  (params (Caller :type BP%20Spline%20Follower%20Component%20Object%20Reference) (FollowingActor :type Actor%20Object%20Reference) (FollowedSpline :type Spline%20Component%20Object%20Reference) (ReachedDistance :type Float%20%28double-precision%29) (ReachedKey :type Float%20%28double-precision%29))
  (Default|CallOnFollowerReachedTargetonSpline FollowingActor Caller ReachedKey))

(event EventActorStartedFollowingSpline
  (params (FollowingActor :type Actor%20Object%20Reference) (FollowerComponent :type BP%20Spline%20Follower%20Component%20Object%20Reference))
  (Utilities|Map|Add (Variables|Default|GetCurrentSplineFollowers) FollowingActor FollowerComponent)
  (Game|AssignOnDestroyed FollowingActor (EventDispatchers|CreateEvent :!event Custom|OnFollowingActorDestroyed))
  (Default|CallOnActorStartedFollowingSpline FollowingActor FollowerComponent)
  (EventDispatchers|BindEventtoOnSplineMovementCompletelyFinished FollowerComponent (EventDispatchers|CreateEvent :!event Custom|FollowerReachedTarget)))

(event EventActorStoppedFollowingSpline
  (params (Actor :type Actor%20Object%20Reference) (SplineFollowComponent :type BP%20Spline%20Follower%20Component%20Object%20Reference))
  (CallFunction|CleanupFollower Actor SplineFollowComponent))

(event EventFollowerPassedNotify
  (params (Actor :type Actor%20Object%20Reference) (FollowComponent :type BP%20Spline%20Follower%20Component%20Object%20Reference) (Notify :type Spline%20Notify%20Struct%20Structure%20%28by%20ref%29))
  (Default|CallOnFollowerPassedNotifyPoint Actor FollowComponent Notify))

(fn ConstructionScript)

(fn CleanupFollower
  (params (FollowerActor :type Actor%20Object%20Reference) (FollowComponent :type BP%20Spline%20Follower%20Component%20Object%20Reference))
  (Utilities|Map|Remove (Variables|Default|GetCurrentSplineFollowers) FollowerActor)
  (Utilities|IsValid FollowComponent
    (:Is%20Valid
      (EventDispatchers|UnbindEventfromOnSplineMovementCompletelyFinished FollowComponent (EventDispatchers|CreateEvent :!event Custom|FollowerReachedTarget))
      (Default|CallOnActorStoppedFollowingSpline FollowerActor FollowComponent))))

(fn GetSplineNotifies
  (return (Variables|Default|GetSplineNotifyPoints)))

(fn GetSplines
  (bind _spline1 (Variables|Default|GetSpline1))
  (return _spline1 _spline1))

(fn IsActoronSpline
  (params (ActorToCheck :type Actor%20Object%20Reference))
  (return (.ReturnValue (Utilities|Map|Find (Variables|Default|GetCurrentSplineFollowers) ActorToCheck))))

(fn IsSplineinUse
  (return (> (Utilities|Map|Length (Variables|Default|GetCurrentSplineFollowers)) 0)))