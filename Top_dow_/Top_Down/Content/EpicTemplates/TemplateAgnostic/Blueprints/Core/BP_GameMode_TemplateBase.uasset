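; Base game mode for templates, handling local multiplayer, player starts, game-over rules and shared level services.
; Split screen is set in the construction script before possession, and BeginPlay creates extra players from the game instance's count.
; Each controller keeps a unique random start, and game over async-loads a menu widget.
; Tagged level bools/ints and actor reuse go through interface-based objects, found or spawned on demand, with value updates relayed.
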(event Custom|DisplayGameOverWidget
  (bind _class (Utilities|AsyncLoadClassAsset (Variables|TemplateGameMode|GetGameOverMenuWidget))
    (:Completed
      (bind _asw_menu_widget (Utilities|Casting|CastToW_MenuWidgetClass _class))
      (bind _returnvalue (UserInterface|CreateWidget _asw_menu_widget (Game|GetPlayerController 0)))
      (CallFunction|DisplayGamewideMenu _returnvalue))))

(event EventEndPlay
  (params (EndPlayReason :type EEndPlayReason%20Enum :default "Destroyed"))
  (Class|GameplayStatics|SetForceDisableSplitscreen false))

(event EventBeginPlay
  (|CallParentFunction)
  (CallFunction|SpawninAdditionalPlayersifRequired))

(fn ConstructionScript
  (Class|GameplayStatics|SetForceDisableSplitscreen (Utilities|Enum|Equal(Enum) (Variables|TemplateGameMode|GetMultiplayerMode) "NewEnumerator2")) ; We do this here, rather than BeginPlay, so that this value is setup BEFORE any controllers possess their pawns.\nThose pawns might need to know if split screen is enabled for certain logic (such as controlling spline offset)
)

(fn TryGetLevelBool
  (params (LevelBoolTag :type Gameplay%20Tag%20Structure))
  (Utilities|GetLevelDataSource
    (:Succeeded
      (bind (_boolvalue _isvalid) (Class|BPIGameplayLevelDataSource|TryGetLevelBool(Message) (Variables|TemplateGameMode|GetGameplayLevelDataSource) LevelBoolTag))
      (return _boolvalue _isvalid))
    (:Failed
      (Development|PrintString (Utilities|String|Append "BP_GameMode_TemplateBase::GetLevelBool '" (GameplayTags|GetDebugStringfromGameplayTag LevelBoolTag) "' failed because no GameplayLevelDataSource is assigned."))
      (return false false))))

(fn TryGetLevelInt
  (params (LevelIntTag :type Gameplay%20Tag%20Structure))
  (Utilities|GetLevelDataSource
    (:Succeeded
      (bind (_intvalue _isvalid) (Class|BPIGameplayLevelDataSource|TryGetLevelInt(Message) (Variables|TemplateGameMode|GetGameplayLevelDataSource) LevelIntTag))
      (return _intvalue _isvalid))
    (:Failed
      (Development|PrintString (Utilities|String|Append "BP_GameMode_TemplateBase::GetLeveInt '" (GameplayTags|GetDebugStringfromGameplayTag LevelIntTag) "' failed because no GameplayLevelDataSource is assigned."))
      (return 0 false))))

(fn SetLevelBool
  (params (LevelBoolTag :type Gameplay%20Tag%20Structure) (NewValue :type Boolean))
  (Utilities|GetLevelDataSource
    (:Succeeded
      (Class|BPIGameplayLevelDataSource|SetLevelBool(Message) (Variables|TemplateGameMode|GetGameplayLevelDataSource) LevelBoolTag NewValue))
    (:Failed
      (Development|PrintString (Utilities|String|Append "BP_GameMode_TemplateBase::GetLevelBool '" (GameplayTags|GetDebugStringfromGameplayTag LevelBoolTag) "' failed because no GameplayLevelDataSource is assigned.")))))

(fn SetLevelInt
  (params (LevelIntTag :type Gameplay%20Tag%20Structure) (NewValue :type Integer))
  (Utilities|GetLevelDataSource
    (:Succeeded
      (Class|BPIGameplayLevelDataSource|SetLevelInt(Message) (Variables|TemplateGameMode|GetGameplayLevelDataSource) LevelIntTag NewValue))
    (:Failed
      (Development|PrintString (Utilities|String|Append "BP_GameMode_TemplateBase::GetLevelBool '" (GameplayTags|GetDebugStringfromGameplayTag LevelIntTag) "' failed because no GameplayLevelDataSource is assigned.")))))

(fn UpdateGameplayLevelDataSource
  (params (NewGameplayLevelDataSource :type Object%20Object%20Reference))
  (if (== NewGameplayLevelDataSource (Variables|TemplateGameMode|GetGameplayLevelDataSource))
    (return)
    (elif (Utilities|DoesObjectImplementInterface NewGameplayLevelDataSource "/Game/EpicTemplates/TemplateAgnostic/Blueprints/Interfaces/BPI_GameplayLevelDataSource.BPI_GameplayLevelDataSource_C")
      (Utilities|IsValid (Variables|TemplateGameMode|GetGameplayLevelDataSource)
        (:Is%20Valid
          (Development|PrintString (Utilities|String|Append "GameMode_TemplateBase::UpdateGameplayLevelDataSource - Trying to assign a new data source '" (Utilities|GetDisplayName NewGameplayLevelDataSource) "' when '" (Utilities|GetDisplayName (Variables|TemplateGameMode|GetGameplayLevelDataSource)) "' is already assigned")))
        (:Is%20Not%20Valid
          (Variables|TemplateGameMode|SetGameplayLevelDataSource NewGameplayLevelDataSource)))
      (else
        (Development|PrintString (Utilities|String|Append "GameMode_TemplateBase::UpdateGameplayLevelDataSource - Trying to assign a new data source '" (Utilities|GetDisplayName NewGameplayLevelDataSource) "' but it doesn't implement the BPi_GameplayDataSource interface"))))))

(fn TryFindLevelDataSource
  (bind _outactors (Actor|GetAllActorswithInterface "/Game/EpicTemplates/TemplateAgnostic/Blueprints/Interfaces/BPI_GameplayLevelDataSource.BPI_GameplayLevelDataSource_C"))
  (if (> (Utilities|Array|Length _outactors) 0)
    (Variables|TemplateGameMode|SetGameplayLevelDataSource (Utilities|Array|Get(acopy) _outactors))
    (return true)
    (else
      (bind _returnvalue (Game|SpawnActorfromClass "/Game/EpicTemplates/TemplateAgnostic/Blueprints/BP_GameplayLevelData.BP_GameplayLevelData_C" (Math|Transform|MakeTransform "0, 0, 0") "AlwaysSpawn" "MultiplyWithRoot" 0 0))
      (Utilities|IsValid _returnvalue
        (:Is%20Valid
          (Variables|TemplateGameMode|SetGameplayLevelDataSource _returnvalue)
          (return true))
        (:Is%20Not%20Valid
          (return false))))))

(fn NotifyLevelBoolValueUpdated
  (params (Source :type BPI%20Gameplay%20Level%20Data%20Source%20Interface) (BoolTag :type Gameplay%20Tag%20Structure))
  (bind _boolvalue (Default|TryGetLevelBool Source BoolTag))
  (Default|CallOnLevelBoolUpdated BoolTag _boolvalue))

(fn NotifyLevelIntValueUpdated
  (params (Source :type BPI%20Gameplay%20Level%20Data%20Source%20Interface) (IntTag :type Gameplay%20Tag%20Structure))
  (bind _intvalue (Default|TryGetLevelInt Source IntTag))
  (Default|CallOnLevelIntUpdated IntTag _intvalue))

(fn GetActorReuseManager
  (bind _fallbackactoreusemanagerclass (Variables|TemplateGameMode|GetFallbackActoReuseManagerClass))
  (if (Utilities|IsValidInterface (Variables|TemplateGameMode|GetActorReuseManager))
    (return (Variables|TemplateGameMode|GetActorReuseManager))
    (else
      (bind _returnvalue (Utilities|LoadClassAssetBlocking _fallbackactoreusemanagerclass))
      (bind _asactor (Utilities|Casting|CastToActorClass _returnvalue))
      (if (Class|KismetSystemLibrary|DoesClassImplementInterface _asactor "/Game/EpicTemplates/TemplateAgnostic/Blueprints/Interfaces/BPI_ActorReuseManager.BPI_ActorReuseManager_C")
        (bind _returnvalue_2 (Game|SpawnActorfromClass _asactor (Math|Transform|MakeTransform "0.000000,0.000000,-1000.000000") "AlwaysSpawn" "MultiplyWithRoot" 0 0))
        (bind _output_get (Variables|TemplateGameMode|SetCachedActorReuseManagerActor _returnvalue_2))
        (bind _asbpi_actor_reuse_manager (Utilities|Casting|CastToBPI_ActorReuseManager _output_get))
        (bind _output_get_2 (Variables|TemplateGameMode|SetActorReuseManager _asbpi_actor_reuse_manager))
        (return _output_get_2)
        (else
          (Development|PrintString (Utilities|String|Append "BP_GameMode_TemplateBase::GetActorReuseManager - FallbackActorReuseManagerClass '" (Utilities|ToString(SoftClassReference) _fallbackactoreusemanagerclass) "' does not implement the BPI_ActorReuseManager interface, and is therefore not suitable"))
          (return 0))))))

(fn CheckforGameOver
  (for _index (range 0 (- (Class|GameplayStatics|GetNumLocalPlayerControllers) 1))
    (bind _output_get (LocalVariables|SetCurrentPlayerIndex _index))
    (LocalVariables|SetCurrentPlayerCont (Game|GetPlayerController _output_get))
    (switch Utilities|FlowControl|Switch|SwitchonEGameOverRule (Variables|TemplateGameMode|GetGameOverRule)
      (:NewEnumerator0
        (bind _bisplayeralive (TemplateGameMode|Protected|IsPlayerControllerAlive (LocalVariables|GetCurrentPlayerCont)))
        (if (not _bisplayeralive)
          (TemplateGameMode|Protected|GameOver)))
      (:NewEnumerator1
        (bind _bisplayeralive_2 (TemplateGameMode|Protected|IsPlayerControllerAlive (LocalVariables|GetCurrentPlayerCont)))
        (if (not _bisplayeralive_2)
          (if (== (LocalVariables|GetCurrentPlayerIndex) 0)
            (TemplateGameMode|Protected|GameOver))))
      (:NewEnumerator2
        (bind _bisplayeralive_3 (TemplateGameMode|Protected|IsPlayerControllerAlive (LocalVariables|GetCurrentPlayerCont)))
        (if _bisplayeralive_3
          (return)
          (elif (== (LocalVariables|GetCurrentPlayerIndex) (- (Class|GameplayStatics|GetNumLocalPlayerControllers) 1))
            (TemplateGameMode|Protected|GameOver)))))))

(fn IsPlayerControllerAlive
  (params (PlayerController :type Player%20Controller%20Object%20Reference))
  (if (Utilities|DoesObjectImplementInterface PlayerController "/Game/EpicTemplates/TemplateAgnostic/Blueprints/Interfaces/BPI_PlayerAliveSource.BPI_PlayerAliveSource_C")
    (bind _bisplayeralive (Class|BPIPlayerAliveSource|IsPlayerAlive(Message) PlayerController))
    (return _bisplayeralive)
    (else
      (Development|PrintString (Utilities|String|Append "Player controller '" (Utilities|GetDisplayName PlayerController) "' doesn't implement BPi_PlayerAlive interface, assuming Player Is Alive"))
      (return true))))

(fn GameOver
  (if (not (Variables|TemplateGameMode|GetbGameIsOver))
    (Variables|TemplateGameMode|SetbGameIsOver true)
    (CallFunction|DisplayGameOverWidget)))

(fn IsGameOver
  (return (Variables|TemplateGameMode|GetbGameIsOver)))

(fn FindPlayerStart
  (params (Player :type Controller%20Object%20Reference) (IncomingName :type String))
  (Utilities|FlowControl|Sequence
    (:then_0
      (if (Utilities|Array|IsEmpty (Variables|TemplateGameMode|GetPlayerStarts))
        (bind _outactors (Actor|GetAllActorsOfClass "/Script/Engine.PlayerStart"))
        (Variables|TemplateGameMode|SetPlayerStarts _outactors)))
    (:then_1
      (bind _output_get (LocalVariables|SetChosenStart (.Value (Utilities|Map|Find (Variables|TemplateGameMode|GetControllerToStartMapping) Player))))
      (Utilities|IsValid _output_get
        (:Is%20Valid
          (return (LocalVariables|GetChosenStart)))
        (:Is%20Not%20Valid
          (if (> (Utilities|Array|Length (Variables|TemplateGameMode|GetPlayerStarts)) 0)
            (bind _output_get_2 (LocalVariables|SetRandomIdx (.OutIndex (Utilities|Array|Random (Variables|TemplateGameMode|GetPlayerStarts)))))
            (LocalVariables|SetChosenStart (Utilities|Array|Get(acopy) (Variables|TemplateGameMode|GetPlayerStarts) _output_get_2))
            (Utilities|Array|RemoveIndex (Variables|TemplateGameMode|GetPlayerStarts) (LocalVariables|GetRandomIdx))
            (Utilities|Map|Add (Variables|TemplateGameMode|GetControllerToStartMapping) Player (LocalVariables|GetChosenStart))
            (return (LocalVariables|GetChosenStart))
            (else
              (Development|PrintString (Utilities|String|Append "BP_GameMode_TemplateBase::FindPlayerStart - Not enough player starts to spawn a pawn for player '" (Utilities|GetDisplayName Player) "'. Consider adding more player starts to the level. Reverting to default behaviour.") true true "(R=1.000000,G=0.226237,B=0.000000,A=1.000000)" 2e+01)
              (bind _returnvalue (|CallParentFunction Player IncomingName))
              (return _returnvalue))))))))

(fn GetMultiplayerMode
  (return (Variables|TemplateGameMode|GetMultiplayerMode)))

(fn SpawninAdditionalPlayersifRequired
  (if (Utilities|Enum|NotEqual(Enum) (Variables|TemplateGameMode|GetMultiplayerMode) "NewEnumerator0")
    (bind _asbp_game_instance (Utilities|Casting|CastToBP_GameInstance (Game|GetGameInstance)))
    (if (> (Default|GetNumberOfPlayers _asbp_game_instance) 1)
      (LocalVariables|SetCurrentLocalPlayers (Class|GameplayStatics|GetNumLocalPlayerControllers))
      (for _index (range 0 (- (- (Default|GetNumberOfPlayers _asbp_game_instance) (LocalVariables|GetCurrentLocalPlayers)) 1))
        (Class|GameplayStatics|CreatePlayer -1)))))