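; BP_WallActor is an invisible wall actor that sizes and places a collision box along the line between two corner points.
; UpdateLocationAndExtentsForCorners centers the actor between the corners, aligns its X axis to the segment, raises it by half height and shifts it sideways by half depth.
; The side of that shift follows corner order, via a cross product with up.
; UpdateExtents then resizes the root box to the segment length and preset depth and height.
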(event Custom|UpdateExtents
  (params (InBoxExtent :type Vector))
  (Components|Box|SetBoxExtent (Variables|Default|GetCollisionBoxRoot) InBoxExtent true))

(fn ConstructionScript)

(fn UpdateLocationandExtentsforCorners
  (params (Corner1 :type Vector%20%28by%20ref%29) (Corner2 :type Vector%20%28by%20ref%29))
  (bind _output_get (LocalVariables|SetCornerOffset (- Corner2 Corner1)))
  (bind _output_get_2 (LocalVariables|SetOffsetLength (Math|Vector|VectorLength _output_get)))
  (LocalVariables|SetOffsetDirection (/ (LocalVariables|GetCornerOffset) _output_get_2))
  (Transformation|SetActorTransform self (Math|Transform|MakeTransform (+ (+ Corner1 (* (LocalVariables|GetCornerOffset) 0.5)) (* (Math|Vector|CrossProduct (LocalVariables|GetOffsetDirection) "0.000000,0.000000,1.000000") (LocalVariables|GetInvisibleWallHalfDepth)) (Math|Vector|MakeVector 0.0 0.0 (LocalVariables|GetInvisibleWallHalfHeight))) (Math|Rotator|MakeRotfromX (LocalVariables|GetOffsetDirection))))
  (CallFunction|UpdateExtents self (Math|Vector|MakeVector (* (LocalVariables|GetOffsetLength) 0.5) (LocalVariables|GetInvisibleWallHalfDepth) (LocalVariables|GetInvisibleWallHalfHeight))))