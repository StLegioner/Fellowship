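; BP_CinematicTrigger is a box trigger that plays a Level Sequence when a player-controlled pawn overlaps it, optionally only once.
; It plays a placed sequence actor if valid, otherwise loads the sequence asset, async or blocking, and creates a player for it.
; Cinematic mode can be applied to all local player controllers during playback; on finish it is released and OnCinematicFinished is broadcast.
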(event OnComponentBeginOverlap(CollisionBox)
  (params (OverlappedComponent :type Primitive%20Component%20Object%20Reference) (OtherActor :type Actor%20Object%20Reference) (OtherComp :type Primitive%20Component%20Object%20Reference) (OtherBodyIndex :type Integer) (bFromSweep :type Boolean) (SweepResult :type Hit%20Result%20Structure%20%28by%20ref%29))
  (bind _aspawn (Utilities|Casting|CastToPawn OtherActor))
  (if (Pawn|IsPlayerControlled _aspawn)
    (CallFunction|PlayCinematic)))

(event Custom|PlayCinematic
  (bind _sequenceactor (Variables|CinematicTrigger|GetSequenceActor))
  (bind _output (Utilities|ResolveSoftReference _sequenceactor))
  (if (or (not (Variables|CinematicTrigger|GetbOnlyPlayOnce)) (not (Variables|CinematicTrigger|GetbHasPlayed)))
    (Variables|CinematicTrigger|SetbHasPlayed true)
    (Utilities|FlowControl|Sequence
      (:then_0
        (if (Variables|CinematicTrigger|GetbOnlyPlayOnce)
          (Collision|SetActorEnableCollision false)))
      (:then_1
        (if (Variables|CinematicTrigger|GetbEnterCinematicModeOnPlay)
          (CallFunction|EnterCinematicMode)))
      (:then_2
        (Utilities|IsValid _output
          (:Is%20Valid
            (CallFunction|BindtoFinishedandPlay (Variables|/Script/LevelSequence.LevelSequenceActor|GetSequencePlayer _output)))
          (:Is%20Not%20Valid
            (if (Variables|CinematicTrigger|GetbLoadSequenceAssetAsync)
              (bind _object (Utilities|AsyncLoadAsset (Variables|CinematicTrigger|GetSequenceAsset))
                (:Completed
                  (bind _aslevel_sequence (Utilities|Casting|CastToLevelSequence _object))
                  (bind _returnvalue (Sequencer|Player|CreateLevelSequencePlayer _aslevel_sequence))
                  (CallFunction|BindtoFinishedandPlay _returnvalue)))
              (else
                (bind _returnvalue_2 (Utilities|LoadAssetBlocking (Variables|CinematicTrigger|GetSequenceAsset)))
                (bind _aslevel_sequence_2 (Utilities|Casting|CastToLevelSequence _returnvalue_2))
                (bind _returnvalue_3 (Sequencer|Player|CreateLevelSequencePlayer _aslevel_sequence_2))
                (CallFunction|BindtoFinishedandPlay _returnvalue_3)))))))))

(event Custom|UpdateTriggerEnabled
  (params (IsEnabled :type Boolean))
  (Collision|SetCollisionEnabled (Variables|Default|GetCollisionBox) (select IsEnabled "QueryOnly" "NoCollision")))

(event Custom|CinematicFinished
  (Utilities|FlowControl|Sequence
    (:then_0
      (if (Variables|CinematicTrigger|GetbEnterCinematicModeOnPlay)
        (CallFunction|LeaveCinematicMode)))
    (:then_1
      (Default|CallOnCinematicFinished self))))

(event Custom|BindToFinishedAndPlay
  (params (SequencePlayer :type Movie%20Scene%20Sequence%20Player%20Object%20Reference))
  (EventDispatchers|BindEventtoOnFinished SequencePlayer (delegate Custom|CinematicFinished))
  (Sequencer|Player|Play SequencePlayer :!class /Script/MovieScene.MovieSceneSequencePlayer))

(fn ConstructionScript
  (Components|Box|SetBoxExtent (Variables|Default|GetCollisionBox) (* (Variables|CinematicTrigger|GetCollisionSize) 0.5) true)
  (Collision|SetCollisionEnabled (Variables|Default|GetCollisionBox) (select (Variables|CinematicTrigger|GetbStartTriggerEnabled) "QueryOnly" "NoCollision")))

(fn EnterCinematicMode
  (bind _output_get (LocalVariables|SetPlayerControllerCount (Class|GameplayStatics|GetNumLocalPlayerControllers)))
  (for _index (range 0 (- _output_get 1))
    (Class|PlayerController|SetCinematicMode (Game|GetPlayerController _index) true (Variables|CinematicTrigger|GetbHidePlayer) true true true)))

(fn LeaveCinematicMode
  (bind _output_get (LocalVariables|SetPlayerControllerCount (Class|GameplayStatics|GetNumLocalPlayerControllers)))
  (for _index (range 0 (- _output_get 1))
    (Class|PlayerController|SetCinematicMode (Game|GetPlayerController _index) false true true true true)))