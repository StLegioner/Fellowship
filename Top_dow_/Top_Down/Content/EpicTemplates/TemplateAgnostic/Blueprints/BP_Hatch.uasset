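; BP_Hatch is a hatch actor that breaks when its health component reports damage.
; On damage it disables mesh collision, spawns a BP_DestructableHatch at its transform, passes on its velocity as an impulse and applies the hit at the damage location.
; It then signals its destruction through CallOnHatchDestroyed and destroys itself, so the destructible actor replaces the intact one.
; The construction script caches the mesh's default material.
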(event OnTookDamage(BP_HealthComponent)
  (params (Caller :type BP%20Health%20Component%20Object%20Reference) (OldHealth :type Float%20%28double-precision%29) (NewHealth :type Float%20%28double-precision%29) (SpecialDamageName :type Name :default "None") (DamageStruct :type Damage%20Struct%20Structure))
  (Collision|SetCollisionEnabled (Variables|Default|GetMesh) "NoCollision")
  (bind _returnvalue (Game|SpawnActorfromClass "/Game/EpicTemplates/TemplateAgnostic/DestructableMeshes/BP_DestructableHatch.BP_DestructableHatch_C" (Transformation|GetActorTransform) "Undefined" "MultiplyWithRoot" 0 0))
  (Default|AddImpulse _returnvalue (Transformation|GetVelocity))
  (Default|ApplyHit _returnvalue (.DamageLocation (Utilities|Struct|BreakDamageStruct DamageStruct)))
  (Default|CallOnHatchDestroyed)
  (Actor|DestroyActor))

(fn ConstructionScript
  (Variables|HatchProperties|SetDefaultMeshMaterial (Rendering|Material|GetMaterial (Variables|Default|GetMesh) 0)))