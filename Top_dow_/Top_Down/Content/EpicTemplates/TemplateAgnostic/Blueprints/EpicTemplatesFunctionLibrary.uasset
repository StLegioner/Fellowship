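; Shared Blueprint function library for the Epic templates, giving static helpers for menus, players, scores, level flags, input prompts, cinematics and cameras.
; Most gameplay helpers forward to the template game mode, game instance or player controller via casts, including pooled actor spawning through the reuse manager.
; A recursive interface search over actors, components and child actors underpins spline and score lookups.
; Camera math projects the view frustum onto planes and clamps positions within 2D bounds.
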(fn SearchActorforInterface
  (params (Actor :type Actor%20Object%20Reference) (Interface :type Interface%20Class%20Reference) (SearchChildActorComponents :type Boolean))
  (Utilities|IsValid Actor
    (:Is%20Valid
      (if (Utilities|DoesObjectImplementInterface Actor Interface)
        (return Actor true)
        (else
          (bind _output_get (LocalVariables|SetImplementingComponents (Class|Actor|GetComponentsbyInterface Actor Interface)))
          (if (> (Utilities|Array|Length _output_get) 0)
            (return (Utilities|Array|Get(acopy) (LocalVariables|GetImplementingComponents)) true)
            (elif SearchChildActorComponents
              (for _array_element (Actor|GetAllChildActors Actor false)
                (bind (_interfaceimplementingobject _foundimplementingobject) (EpicTemplatesFunctionLibrary|Utilities|SearchActorforInterface _array_element Interface true (LocalVariables|Get__WorldContext)))
                (if _foundimplementingobject
                  (return _interfaceimplementingobject true)))
              (return 0 false)
              (else
                (return 0 false)))))))
    (:Is%20Not%20Valid
      (return 0 false))))

(fn PlusEqualsFloat
  (params (InOutFloat :type Float%20%28double-precision%29%20%28by%20ref%29) (Addition :type Float%20%28double-precision%29))
  (|SetBy-RefVar InOutFloat (+ InOutFloat Addition))
  (return InOutFloat))

(fn MinusEqualsFloat
  (params (InOutFloat :type Float%20%28double-precision%29%20%28by%20ref%29) (Subtraction :type Float%20%28double-precision%29))
  (|SetBy-RefVar InOutFloat (- InOutFloat Subtraction))
  (return InOutFloat))

(fn PlusEqualsInt
  (params (InOutInt :type Integer%20%28by%20ref%29) (Addition :type Integer))
  (|SetBy-RefVar InOutInt (+ InOutInt Addition))
  (return InOutInt))

(fn MinusEqualsInt
  (params (InOutInt :type Integer%20%28by%20ref%29) (Subtraction :type Integer))
  (|SetBy-RefVar InOutInt (- InOutInt Subtraction))
  (return InOutInt))

(fn DisplayGamewideMenu
  (params (Menu :type W%20Menu%20Widget%20Object%20Reference))
  (UserInterface|Viewport|AddtoViewport Menu 0)
  (Class|BPIMenuManipulator|MenuBeingDisplayed(Message) (Game|GetPlayerController 0) Menu))

(fn DisplayPlayerMenu
  (params (Menu :type W%20Menu%20Widget%20Object%20Reference) (PlayerIndex :type Integer))
  (UserInterface|Viewport|AddtoPlayerScreen Menu)
  (Class|BPIMenuManipulator|MenuBeingDisplayed(Message) (Game|GetPlayerController 0 PlayerIndex) Menu))

(fn GetSplinesfromActor
  (params (SplineActor :type Actor%20Object%20Reference))
  (Utilities|IsValid SplineActor
    (:Is%20Valid
      (Utilities|FlowControl|Sequence
        (:then_0
          (bind _interfaceimplementingobject (EpicTemplatesFunctionLibrary|Utilities|SearchActorforInterface SplineActor "/Game/EpicTemplates/TemplateAgnostic/Blueprints/Interfaces/BPI_SplinePathImplementor.BPI_SplinePathImplementor_C" false))
          (bind _output_get (LocalVariables|SetInterfaceImplementer _interfaceimplementingobject))
          (Utilities|IsValid _output_get
            (:Is%20Valid
              (bind (_pathspline1 _pathspline2) (Class|BPISplinePathImplementor|GetSplines(Message) (LocalVariables|GetInterfaceImplementer)))
              (Utilities|FlowControl|Sequence
                (:then_0
                  (Utilities|IsValid _pathspline1
                    (:Is%20Valid
                      (Utilities|Array|Add (LocalVariables|GetFoundSplines) _pathspline1))))
                (:then_1
                  (Utilities|IsValid _pathspline2
                    (:Is%20Valid
                      (Utilities|Array|Add (LocalVariables|GetFoundSplines) _pathspline2))))))
            (:Is%20Not%20Valid
              (LocalVariables|SetFoundSplines (Actor|GetComponentsByClass SplineActor "/Script/Engine.SplineComponent")))))
        (:then_1
          (return (LocalVariables|GetFoundSplines) (> (Utilities|Array|Length (LocalVariables|GetFoundSplines)) 0)))))
    (:Is%20Not%20Valid
      (return 0 false))))

(fn IsinSinglePlayerMode
  (Utilities|FlowControl|Sequence
    (:then_0
      (bind _asbp_game_instance (Utilities|Casting|CastToBP_GameInstance (Game|GetGameInstance)))
      (LocalVariables|SetbSinglePlayer (== (Default|GetNumberOfPlayers _asbp_game_instance) 1)))
    (:then_1
      (if (not (Class|KismetSystemLibrary|IsPackagedforDistribution))
        ;[1 1 1] This could only happen when jumping in to testing a level without going through the menu flow
        (if (not (LocalVariables|GetbSinglePlayer))
          (bind _asbp_game_mode_template_base (Utilities|Casting|CastToBP_GameMode_TemplateBase (Game|GetGameMode)))
          (LocalVariables|SetbSinglePlayer (Utilities|Enum|Equal(Enum) (Default|GetMultiplayerMode _asbp_game_mode_template_base) "NewEnumerator0")))))
    (:then_2
      (return (LocalVariables|GetbSinglePlayer)))))

(fn GetSaveSlotName
  (return (LocalVariables|GetSaveSlotName)))

(fn FindWidgetGroupIndexforWidget
  (params (InWidgetGroups :type Array%20of%20Widget%20Group%20Struct%20Structures) (Widget :type User%20Widget%20Object%20Reference) (AddToArrayIfNotFound :type Boolean))
  (LocalVariables|SetWidgetClass (Utilities|GetClass Widget))
  (for (_array_element _array_index) InWidgetGroups
    (LocalVariables|SetCurrentIndex _array_index)
    (if (== (.WidgetClass (Utilities|Struct|BreakWidgetGroupStruct _array_element)) (LocalVariables|GetWidgetClass))
      (return (LocalVariables|GetCurrentIndex))))
  (if AddToArrayIfNotFound
    (bind _returnvalue (Utilities|Array|Add InWidgetGroups (Utilities|Struct|MakeWidgetGroupStruct (LocalVariables|GetWidgetClass) (Utilities|Array|MakeArray))))
    (return _returnvalue)
    (else
      (return -1))))

(fn GatherandUpdatePlayerScores
  (Utilities|FlowControl|Sequence
    (:then_0
      (for _index (range 0 (- (Class|GameplayStatics|GetNumPlayerControllers) 1))
        (bind (_interfaceimplementingobject _foundimplementingobject) (EpicTemplatesFunctionLibrary|Utilities|SearchActorforInterface (Game|GetPlayerController 0 _index) "/Game/EpicTemplates/TemplateAgnostic/Blueprints/Interfaces/BPI_GameScoreStorage.BPI_GameScoreStorage_C" false))
        (if _foundimplementingobject
          (bind _currentscore (Class|BPIGameScoreStorage|GetCurrentScore(Message) _interfaceimplementingobject))
          (bind _returnvalue (Game|GetCurrentLevelName 0))
          (Utilities|Array|Add (LocalVariables|GetPlayerScores) (Utilities|Struct|MakeSaveScoreStruct "" _returnvalue _index _currentscore)))))
    (:then_1
      (bind _asbp_game_instance (Utilities|Casting|CastToBP_GameInstance (Game|GetGameInstance))
        (:then
          (bind _output_get (LocalVariables|SetGameInst _asbp_game_instance))
          (Default|UpdatePlayerScores _output_get (LocalVariables|GetPlayerScores)))
        (:CastFailed
          (Development|PrintString 0 "EpicTemplatesFunctionLibrary::GatherAndUpdatePlayerScores - Failed, expected Game instance to inherit from BP_GameInstance, but it didn't" true true "(R=1.000000,G=0.177428,B=0.000000,A=1.000000)" 1e+01))))
    (:then_2
      (return (LocalVariables|GetPlayerScores)))))

(fn GetPlayer1Color
  (return "(R=1.000000,G=0.000000,B=0.000000,A=1.000000)"))

(fn GetPlayer2Color
  (return "(R=0.000000,G=0.000000,B=1.000000,A=1.000000)"))

(fn GetTitleMenu
  (return "/Game/EpicTemplates/GameBootLevel.GameBootLevel"))

(fn TrimExcessPlayers
  (LocalVariables|SetCurrentPlayerIndex (- (Class|GameplayStatics|GetNumLocalPlayerControllers) 1))
  (while (> (LocalVariables|GetCurrentPlayerIndex) 0)
    (Utilities|FlowControl|Sequence
      (:then_0
        (Utilities|IsValid (Class|GameplayStatics|GetPlayerControllerfromID 0 (LocalVariables|GetCurrentPlayerIndex))
          (:Is%20Valid
            (Class|GameplayStatics|RemovePlayer (Class|GameplayStatics|GetPlayerControllerfromID 0 (LocalVariables|GetCurrentPlayerIndex)) false))))
      (:then_1
        (Math|Integer|DecrementInt (LocalVariables|GetCurrentPlayerIndex))))))

(fn TraceUnderCursorbyChannel
  (params (PlayerController :type Player%20Controller%20Object%20Reference) (TraceChannel :type ETraceTypeQuery%20Enum :default "TraceTypeQuery1") (TraceDistance :type Float%20%28single-precision%29) (bTraceComplex :type Boolean))
  (Utilities|IsValid PlayerController
    (:Is%20Valid
      (if (Utilities|DoesObjectImplementInterface PlayerController "/Game/EpicTemplates/TemplateAgnostic/Blueprints/Interfaces/BPI_CursorImplementor.BPI_CursorImplementor_C")
        (bind _screenpos (Class|BPICursorImplementor|GetCursorScreenPosition(Message) PlayerController))
        (bind (_outhit _returnvalue) (Collision|LineTraceByChannel 0 (.WorldPosition (Class|GameplayStatics|DeprojectScreentoWorld PlayerController _screenpos)) (+ (.WorldPosition (Class|GameplayStatics|DeprojectScreentoWorld PlayerController _screenpos)) (* (.WorldDirection (Class|GameplayStatics|DeprojectScreentoWorld PlayerController _screenpos)) TraceDistance)) TraceChannel bTraceComplex (Utilities|Array|MakeArray (Pawn|GetControlledPawn PlayerController)) "None"))
        (return _outhit _returnvalue)
        (else
          (Development|PrintString 0 (Utilities|String|Append "EpicTemplatesFunctionLibrary::TraceUnderCursorByChannel - Provided player controller '" (Utilities|GetDisplayName PlayerController) "' does not implement the BPi_CursorImplementer interface, so this logic will not work."))
          (return "" false))))
    (:Is%20Not%20Valid
      (return "" false))))

(fn TryGetLevelBool
  (params (LevelBoolTag :type Gameplay%20Tag%20Structure))
  (bind _asbp_game_mode_template_base (Utilities|Casting|CastToBP_GameMode_TemplateBase (Game|GetGameMode))
    (:then
      (bind (_boolvalue _isvalid) (Default|TryGetLevelBool _asbp_game_mode_template_base LevelBoolTag))
      (return _boolvalue _isvalid))
    (:CastFailed
      (Development|PrintString 0 "EpicTemplateFunctionLibrary::TryGetLevelBool - get failed, game mode does not extend from BP_GameMode_TemplateBase" true true "(R=1.000000,G=0.145770,B=0.000000,A=1.000000)" 2e+01))))

(fn TryGetLevelInt
  (params (LevelIntTag :type Gameplay%20Tag%20Structure))
  (bind _asbp_game_mode_template_base (Utilities|Casting|CastToBP_GameMode_TemplateBase (Game|GetGameMode))
    (:then
      (bind (_intvalue _isvalid) (Default|TryGetLevelInt _asbp_game_mode_template_base LevelIntTag))
      (return _intvalue _isvalid))
    (:CastFailed
      (Development|PrintString 0 "EpicTemplateFunctionLibrary::TryGetLevelnt - get failed, game mode does not extend from BP_GameMode_TemplateBase" true true "(R=1.000000,G=0.145770,B=0.000000,A=1.000000)" 2e+01))))

(fn SetLevelBool
  (params (LevelBoolTag :type Gameplay%20Tag%20Structure) (NewValue :type Boolean))
  (bind _asbp_game_mode_template_base (Utilities|Casting|CastToBP_GameMode_TemplateBase (Game|GetGameMode))
    (:then
      (Default|SetLevelBool _asbp_game_mode_template_base LevelBoolTag NewValue))
    (:CastFailed
      (Development|PrintString 0 "EpicTemplateFunctionLibrary::SetLevelBool - set failed, game mode does not extend from BP_GameMode_TemplateBase" true true "(R=1.000000,G=0.145770,B=0.000000,A=1.000000)" 2e+01))))

(fn SetLevelInt
  (params (LevelIntTag :type Gameplay%20Tag%20Structure) (NewValue :type Integer))
  (bind _asbp_game_mode_template_base (Utilities|Casting|CastToBP_GameMode_TemplateBase (Game|GetGameMode))
    (:then
      (Default|SetLevelInt _asbp_game_mode_template_base LevelIntTag NewValue))
    (:CastFailed
      (Development|PrintString 0 "EpicTemplateFunctionLibrary::SetLevelInt - set failed, game mode does not extend from BP_GameMode_TemplateBase" true true "(R=1.000000,G=0.145770,B=0.000000,A=1.000000)" 2e+01))))

(fn BindtoPlayerInputMethodChanged
  (params (PlayerController :type Player%20Controller%20Object%20Reference) (Event :type Delegate%20%28by%20ref%29) (callOnBind :type Boolean))
  (bind _asbp_template_player_controller (Utilities|Casting|CastToBP_TemplatePlayerController PlayerController)
    (:then
      (Default|BindEventtoInputMethodChanged _asbp_template_player_controller callOnBind Event)
      (return true))
    (:CastFailed
      (return false))))

(fn UnbindfromPlayerInputMethodChanged
  (params (PlayerController :type Player%20Controller%20Object%20Reference) (Event :type Delegate%20%28by%20ref%29))
  (bind _asbp_template_player_controller (Utilities|Casting|CastToBP_TemplatePlayerController PlayerController))
  (Default|UnbindEventfromInputMethodChanged _asbp_template_player_controller Event))

(fn DisplayButtonPromptforPlayer
  (params (Controller :type Controller%20Object%20Reference) (PromptID :type Name%20%28by%20ref%29) (NewInputAction :type Input%20Action%20Object%20Reference) (PromptText :type Text) (PromptLocation :type EPromptLocation%20Enum :default "NewEnumerator0"))
  (bind _asbp_template_player_controller (Utilities|Casting|CastToBP_TemplatePlayerController Controller))
  (Default|DisplayButtonPrompt _asbp_template_player_controller PromptID NewInputAction PromptText PromptLocation))

(fn HideButtonPromptforPlayer
  (params (Controller :type Controller%20Object%20Reference) (PromptID :type Name%20%28by%20ref%29))
  (bind _asbp_template_player_controller (Utilities|Casting|CastToBP_TemplatePlayerController Controller))
  (Default|HideButtonPrompt _asbp_template_player_controller PromptID))

(fn SpawnReusableActorfromSoftClassBlocking
  (params (SoftActorClass :type Actor%20Soft%20Class%20Reference) (ActorTrans :type Transform%20%28by%20ref%29) (InOwner :type Actor%20Object%20Reference) (InInstigator :type Pawn%20Object%20Reference))
  (bind _asbp_game_mode_template_base (Utilities|Casting|CastToBP_GameMode_TemplateBase (Game|GetGameMode))
    (:then
      (bind _actorreusemanager (Default|GetActorReuseManager _asbp_game_mode_template_base))
      (bind _actorinstance (Default|RequestActorInstanceSoftBlocking _actorreusemanager SoftActorClass ActorTrans InOwner InInstigator))
      (return _actorinstance true))
    (:CastFailed
      (Development|PrintString 0 "EpicTemplateFunctionLibrary::SpawnRecyclableActor - Spawn failed, game mode does not extend from BP_GameMode_TemplateBase" true true "(R=1.000000,G=0.145770,B=0.000000,A=1.000000)" 2e+01)
      (return 0 false))))

(fn SpawnReusableActorfromClass
  (params (ActorClass :type Actor%20Class%20Reference) (ActorTrans :type Transform%20%28by%20ref%29) (InOwner :type Actor%20Object%20Reference) (InInstigator :type Pawn%20Object%20Reference))
  (bind _asbp_game_mode_template_base (Utilities|Casting|CastToBP_GameMode_TemplateBase (Game|GetGameMode))
    (:then
      (bind _actorreusemanager (Default|GetActorReuseManager _asbp_game_mode_template_base))
      (bind _actorinstance (Default|RequestActorInstance _actorreusemanager ActorClass ActorTrans InOwner InInstigator))
      (return _actorinstance true))
    (:CastFailed
      (Development|PrintString 0 "EpicTemplateFunctionLibrary::SpawnRecyclableActor - Spawn failed, game mode does not extend from BP_GameMode_TemplateBase" true true "(R=1.000000,G=0.145770,B=0.000000,A=1.000000)" 2e+01)
      (return 0 false))))

(fn CalculateCameraViewonPlane
  (params (CameraComponent :type Camera%20Component%20Object%20Reference) (PlaneOrigin :type Vector%20%28by%20ref%29) (PlaneDir :type Vector%20%28by%20ref%29) (MaxViewDistance :type Float%20%28double-precision%29))
  (bind _fieldofview (Variables|/Script/Engine.CameraComponent|GetFieldOfView CameraComponent))
  (bind _returnvalue (* _fieldofview 0.5))
  (bind _returnvalue_2 (Math|Vector|RotateVectorAroundAxis "1.000000,0.000000,0.000000" _returnvalue "0.000000,0.000000,1.000000"))
  (bind (_x _y) (Math|Vector|BreakVector _returnvalue_2))
  (LocalVariables|SetCamTrans (Transformation|GetWorldTransform CameraComponent))
  (bind _output_get (LocalVariables|SetFrustumXYRight (Math|Vector2D|MakeVector2D _x _y)))
  (LocalVariables|SetFrustumXYLeft (* _output_get "(X=1.000000,Y=-1.000000)"))
  (bind _output_get_2 (LocalVariables|SetFrustrumZTop (/ (.Z (Math|Vector|BreakVector (Math|Vector|RotateVectorAroundAxis "1.000000,0.000000,0.000000" (* (Variables|/Script/Engine.CameraComponent|GetFieldOfView CameraComponent) 0.5) "0.000000,-1.000000,0.000000"))) (Variables|/Script/Engine.CameraComponent|GetAspectRatio CameraComponent))))
  (LocalVariables|SetFrustrumZBottom (* _output_get_2 -1.0))
  (return (Utilities|Struct|MakeCameraRectCornersStruct (EpicTemplatesFunctionLibrary|Maths|GetLinetotoPlane (LocalVariables|GetCamTrans) (Math|Vector|MakeVector (.X (Math|Vector2D|BreakVector2D (LocalVariables|GetFrustumXYLeft))) (.Y (Math|Vector2D|BreakVector2D (LocalVariables|GetFrustumXYLeft))) (LocalVariables|GetFrustrumZTop)) MaxViewDistance PlaneOrigin PlaneDir) (EpicTemplatesFunctionLibrary|Maths|GetLinetotoPlane (LocalVariables|GetCamTrans) (Math|Vector|MakeVector (.X (Math|Vector2D|BreakVector2D (LocalVariables|GetFrustumXYRight))) (.Y (Math|Vector2D|BreakVector2D (LocalVariables|GetFrustumXYRight))) (LocalVariables|GetFrustrumZTop)) MaxViewDistance PlaneOrigin PlaneDir) (EpicTemplatesFunctionLibrary|Maths|GetLinetotoPlane (LocalVariables|GetCamTrans) (Math|Vector|MakeVector (.X (Math|Vector2D|BreakVector2D (LocalVariables|GetFrustumXYRight))) (.Y (Math|Vector2D|BreakVector2D (LocalVariables|GetFrustumXYRight))) (LocalVariables|GetFrustrumZBottom)) MaxViewDistance PlaneOrigin PlaneDir) (EpicTemplatesFunctionLibrary|Maths|GetLinetotoPlane (LocalVariables|GetCamTrans) (Math|Vector|MakeVector (.X (Math|Vector2D|BreakVector2D (LocalVariables|GetFrustumXYLeft))) (.Y (Math|Vector2D|BreakVector2D (LocalVariables|GetFrustumXYLeft))) (LocalVariables|GetFrustrumZBottom)) MaxViewDistance PlaneOrigin PlaneDir))))

(fn GetLinetotoPlane
  (params (Transform :type Transform%20%28by%20ref%29) (LineDir :type Vector%20%28by%20ref%29) (LineLength :type Float%20%28double-precision%29) (PlaneOrigin :type Vector%20%28by%20ref%29) (PlaneNormal :type Vector%20%28by%20ref%29))
  (bind _returnvalue (* LineDir LineLength))
  (bind _returnvalue_2 (Math|Transform|TransformLocation Transform _returnvalue))
  (bind _location (Math|Transform|BreakTransform Transform))
  (bind (_t _intersection _returnvalue_3) (Class|KismetMathLibrary|LinePlaneIntersectionOriginNormal _location _returnvalue_2 PlaneOrigin PlaneNormal))
  (return (select _returnvalue_3 _intersection _returnvalue_2)))

(fn Vector2DMax
  (params (Vector1 :type Vector%202D%20Structure%20%28by%20ref%29) (Vector2 :type Vector%202D%20Structure%20%28by%20ref%29))
  (return (Math|Vector2D|MakeVector2D (Math|Float|Max(Float) (.x Vector1) (.x Vector2)) (Math|Float|Max(Float) (.y Vector1) (.y Vector2)))))

(fn Vector2DMin
  (params (Vector1 :type Vector%202D%20Structure%20%28by%20ref%29) (Vector2 :type Vector%202D%20Structure%20%28by%20ref%29))
  (return (Math|Vector2D|MakeVector2D (Math|Float|Min(Float) (.x Vector1) (.x Vector2)) (Math|Float|Min(Float) (.y Vector1) (.y Vector2)))))

(fn GetActorReuseManager
  (bind _asbp_game_mode_template_base (Utilities|Casting|CastToBP_GameMode_TemplateBase (Game|GetGameMode))
    (:then
      (bind _actorreusemanager (Default|GetActorReuseManager _asbp_game_mode_template_base))
      (return _actorreusemanager))
    (:CastFailed
      (Development|PrintString 0 "EpicTemplateFunctionLibrary::GetActorReuseManager - Request failed, game mode does not extend from BP_GameMode_TemplateBase" true true "(R=1.000000,G=0.145770,B=0.000000,A=1.000000)" 2e+01)
      (return 0))))

(fn CinematicStarted(Templates)
  (params (bHideAttachedMeshes :type Boolean) (bHideUI :type Boolean))
  (bind _outactors (Actor|GetAllActorswithInterface 0 "/Game/EpicTemplates/TemplateAgnostic/Blueprints/Interfaces/BPI_CinematicEntity.BPI_CinematicEntity_C"))
  (for _array_element _outactors
    (Class|BPICinematicEntity|UpdateCinematicState(Message) _array_element true bHideAttachedMeshes bHideUI)))

(fn CinematicFinished(Templates)
  (bind _outactors (Actor|GetAllActorswithInterface 0 "/Game/EpicTemplates/TemplateAgnostic/Blueprints/Interfaces/BPI_CinematicEntity.BPI_CinematicEntity_C"))
  (for _array_element _outactors
    (Class|BPICinematicEntity|UpdateCinematicState(Message) _array_element false false false)))

(fn GetClampedLocationAgainstCameraBounds
  (params (DesiredWorldLocation :type Vector%202D%20Structure%20%28by%20ref%29) (PlaneRotation :type Float%20%28double-precision%29) (ViewPlaneWidth :type Float%20%28double-precision%29) (ViewPlaneHeight :type Float%20%28double-precision%29) (WorldCameraBounds2D :type Camera%20Bounds%202D%20Structure%20%28by%20ref%29))
  (bind (_x _y) (Math|Vector2D|BreakVector2D DesiredWorldLocation))
  (bind (_bottombound _bottomboundenforced) (Utilities|Struct|BreakCameraBounds2D WorldCameraBounds2D))
  (bind (_rightbound _rightboundenforced) (Utilities|Struct|BreakCameraBounds2D WorldCameraBounds2D))
  (bind (_leftbound _leftboundenforced) (Utilities|Struct|BreakCameraBounds2D WorldCameraBounds2D))
  (bind (_topbound _topboundenforced) (Utilities|Struct|BreakCameraBounds2D WorldCameraBounds2D))
  (LocalVariables|SetOutputX _x)
  (LocalVariables|SetOutputY _y)
  (LocalVariables|SetWorldSpaceHalfPlaneWidth (* (+ (Math|Float|Absolute(Float) (* (Math|Trig|Cos(Degrees) PlaneRotation) ViewPlaneWidth)) (Math|Float|Absolute(Float) (* (Math|Trig|Sin(Degrees) PlaneRotation) ViewPlaneHeight))) 0.5))
  (LocalVariables|SetWorldSpaceHalfPlaneHeight (* (+ (Math|Float|Absolute(Float) (* (Math|Trig|Sin(Degrees) PlaneRotation) ViewPlaneWidth)) (Math|Float|Absolute(Float) (* (Math|Trig|Cos(Degrees) PlaneRotation) ViewPlaneHeight))) 0.5))
  (Utilities|FlowControl|Sequence
    (:then_0
      (if _rightboundenforced
        (bind _output_get (LocalVariables|SetAdjustedRightBound (- _rightbound (LocalVariables|GetWorldSpaceHalfPlaneWidth))))
        (if (> (LocalVariables|GetOutputX) _output_get)
          (LocalVariables|SetOutputX (LocalVariables|GetAdjustedRightBound))
          (LocalVariables|SetbWantsToBreakRightBound true))))
    (:then_1
      (if _leftboundenforced
        (bind _output_get_2 (LocalVariables|SetAdjustedLeftBound (+ _leftbound (LocalVariables|GetWorldSpaceHalfPlaneWidth))))
        (if (< (LocalVariables|GetOutputX) _output_get_2)
          (if (LocalVariables|GetbWantsToBreakRightBound)
            (LocalVariables|SetOutputX (* (+ (LocalVariables|GetAdjustedLeftBound) (LocalVariables|GetAdjustedRightBound)) 0.5))
            (else
              (LocalVariables|SetOutputX (LocalVariables|GetAdjustedLeftBound)))))))
    (:then_2
      (if _topboundenforced
        (LocalVariables|SetAdjustedTopBound (- _topbound (LocalVariables|GetWorldSpaceHalfPlaneHeight)))
        (if (> (LocalVariables|GetOutputY) (LocalVariables|GetAdjustedTopBound))
          (LocalVariables|SetOutputY (LocalVariables|GetAdjustedTopBound))
          (LocalVariables|SetbWantsToBreakTopBound true))))
    (:then_3
      (if _bottomboundenforced
        (LocalVariables|SetAdjustedBottomBound (+ _bottombound (LocalVariables|GetWorldSpaceHalfPlaneHeight)))
        (if (< (LocalVariables|GetOutputY) (LocalVariables|GetAdjustedBottomBound))
          (if (LocalVariables|GetbWantsToBreakTopBound)
            (LocalVariables|SetOutputY (* (+ (LocalVariables|GetAdjustedBottomBound) (LocalVariables|GetAdjustedTopBound)) 0.5))
            (else
              (LocalVariables|SetOutputY (LocalVariables|GetAdjustedBottomBound)))))))
    (:then_4
      (return (Math|Vector2D|MakeVector2D (LocalVariables|GetOutputX) (LocalVariables|GetOutputY))))))

(fn Get2DCamera
  (bind _asbpi_2dcamera_cache (Utilities|Casting|CastToBPI_2DCameraCache (Game|GetGameMode))
    (:then
      (bind (_cameraactor _camerainterface) (Default|GetCached2DCamera _asbpi_2dcamera_cache))
      (return _cameraactor _camerainterface))
    (:CastFailed
      (return 0 0))))

(fn IsArcadeMachine
  (return (or (Class|KismetSystemLibrary|IsPackagedforDistribution) (LocalVariables|GetTempPretendIsArcadeMachine))))