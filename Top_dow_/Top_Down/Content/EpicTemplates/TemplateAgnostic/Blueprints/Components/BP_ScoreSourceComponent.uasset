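; BP_ScoreSourceComponent is an actor component that gives its owner a score value and a list of score modifiers.
; On BeginPlay it rolls a random integer between the min and max score, or uses the minimum when the max is not higher.
; AddModifier appends to the modifier list, and getters expose the value, the modifiers and the owner's location as the score spawn point.
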(event EventAddModifier
  (params (Modifier :type Score%20Modifier%20Struct%20Structure))
  (Utilities|Array|Add (Variables|ScoreSourceComponent|GetScoreModifiers) Modifier))

(event EventBeginPlay
  (if (> (Variables|ScoreSourceComponent|GetMaxScoreValue) (Variables|ScoreSourceComponent|GetMinScoreValue))
    (Variables|ScoreSourceComponent|SetScoreValue (Math|Random|RandomIntegerinRange (Variables|ScoreSourceComponent|GetMinScoreValue) (Variables|ScoreSourceComponent|GetMaxScoreValue)))
    (else
      (Variables|ScoreSourceComponent|SetScoreValue (Variables|ScoreSourceComponent|GetMinScoreValue)))))

(fn GetModifiers
  (return (Variables|ScoreSourceComponent|GetScoreModifiers)))

(fn GetScoreSpawnLocation
  (return (Transformation|GetActorLocation (Components|GetOwner))))

(fn GetScoreValue
  (return (Variables|ScoreSourceComponent|GetScoreValue)))