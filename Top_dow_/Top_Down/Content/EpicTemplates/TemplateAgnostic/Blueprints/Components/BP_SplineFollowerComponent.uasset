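; Actor component that moves its owner along an attached spline toward a target key, start or end, with pause, lock and debug drawing.
; Each tick it advances a target distance along the spline and snaps, moves or interpolates the owner toward that offset point.
; Placement can sphere-trace for the floor, retrying past initial overlaps, and apply spline rotation per axis.
; Spline notifies crossed between closest input keys are reported through BPI_SplinePathImplementor.
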(event Custom|UpdateSplineFollowOffset
  (params (NewOffset :type Vector) (bSnapToOffset :type Boolean))
  (Variables|SplineFollowerComponent|SetSplineFollowOffset NewOffset)
  (if bSnapToOffset
    (Utilities|IsValid (Variables|SplineFollowerComponent|GetCurrentSpline)
      (:Is%20Valid
        (SplineFollowrComponent|Protected|PlaceOwneratLocation (SplineFollowrComponent|Public|GetOwnerSplineTargetLoc))))))

(event EventBeginPlay
  (SplineFollowrComponent|Protected|SetupCollisionInfo))

(event EventUpdateIsinDebug
  (params (bInIsDebug :type Boolean))
  (Variables|SplineFollowerComponent|SetbInDebugMode bInIsDebug))

(event EventTick
  (params (DeltaSeconds :type Float%20%28single-precision%29))
  (if (not (Variables|SplineFollowerComponent|GetbIsPausedOnSpline))
    (Utilities|FlowControl|Sequence
      (:then_0
        (if (Variables|SplineFollowerComponent|GetbMovingToStartPoint)
          (bind _finishedmoving (SplineFollowrComponent|Public|MoveOwnerTowardsSplineTarget DeltaSeconds))
          (if _finishedmoving
            (Variables|SplineFollowerComponent|SetbMovingToStartPoint false)
            (Default|CallOnReachedStartPoint))
          (else
            (bind _breachedtarget (SplineFollowrComponent|Protected|MoveSplineTarget DeltaSeconds))
            (bind _finishedmoving_2 (SplineFollowrComponent|Public|MoveOwnerTowardsSplineTarget DeltaSeconds))
            (if (and _finishedmoving_2 _breachedtarget)
              (Components|Tick|SetComponentTickEnabled false)
              (Default|CallOnSplineMovementCompletelyFinished self (Components|GetOwner) (Variables|SplineFollowerComponent|GetCurrentSpline) (Variables|SplineFollowerComponent|GetTargetSplineDistance) (Variables|SplineFollowerComponent|GetTargetSplineKey))))))
      (:then_1
        (SplineFollowrComponent|Protected|DebugSplineFollower)))))

(fn AttachtoActorSpline
  (params (SplineComponent :type Spline%20Component%20Object%20Reference) (AttachToSplineType :type EAttachToSplineType%20Enum :default "NewEnumerator0"))
  (if (Variables|SplineFollowerComponent|GetbIsLocked)
    (return)
    (else
      (LocalVariables|SetbReattachingToSameSpline (== SplineComponent (Variables|SplineFollowerComponent|GetCurrentSpline)))
      (Utilities|FlowControl|Sequence
        (:then_0
          (if (not (LocalVariables|GetbReattachingToSameSpline))
            (Utilities|FlowControl|Sequence
              (:then_0
                (if (Utilities|IsValidInterface (Variables|SplineFollowerComponent|GetSplineInterface))
                  (Default|ActorStoppedFollowingSpline (Variables|SplineFollowerComponent|GetSplineInterface) (Components|GetOwner) self)))
              (:then_1
                (Utilities|IsValid SplineComponent
                  (:Is%20Valid
                    (bind _output_get (Variables|SplineFollowerComponent|SetCurrentSpline SplineComponent))
                    (bind _interfaceimplementingobject (CallFunction|SearchActorforInterface (Components|GetOwner _output_get) "/Game/EpicTemplates/TemplateAgnostic/Blueprints/Interfaces/BPI_SplinePathImplementor.BPI_SplinePathImplementor_C" false))
                    (bind _output_get_2 (Variables|SplineFollowerComponent|SetSplineInterfaceObject _interfaceimplementingobject))
                    (Utilities|IsValid _output_get_2
                      (:Is%20Valid
                        (bind _asbpi_spline_path_implementor (Utilities|Casting|CastToBPI_SplinePathImplementor (Variables|SplineFollowerComponent|GetSplineInterfaceObject)))
                        (bind _output_get_3 (Variables|SplineFollowerComponent|SetSplineInterface _asbpi_spline_path_implementor))
                        (bind _notifies (Default|GetSplineNotifies _output_get_3))
                        (Variables|SplineFollowerComponent|SetCurrentSplineNotifies _notifies))
                      (:Is%20Not%20Valid
                        (Variables|SplineFollowerComponent|SetSplineInterface 0)
                        (Utilities|Array|Clear (Variables|SplineFollowerComponent|GetCurrentSplineNotifies)))))
                  (:Is%20Not%20Valid
                    (Variables|SplineFollowerComponent|SetCurrentSpline 0)
                    (Variables|SplineFollowerComponent|SetSplineInterfaceObject 0)
                    (Variables|SplineFollowerComponent|SetSplineInterface 0)
                    (Utilities|Array|Clear (Variables|SplineFollowerComponent|GetCurrentSplineNotifies))))))))
        (:then_1
          (Utilities|IsValid (Variables|SplineFollowerComponent|GetCurrentSpline)
            (:Is%20Valid
              (Utilities|FlowControl|Sequence
                (:then_0
                  (Variables|SplineFollowerComponent|SetVirtualOwnerLocation (Transformation|GetActorLocation (Components|GetOwner)))
                  (LocalVariables|SetClosestKey (Class|SplineComponent|FindInputKeyClosesttoWorldLocation (Variables|SplineFollowerComponent|GetCurrentSpline) (Variables|SplineFollowerComponent|GetVirtualOwnerLocation)))
                  (Variables|SplineFollowerComponent|SetVirtualOwnerLocation (Math|Vector|MakeVector (.x (Variables|SplineFollowerComponent|GetVirtualOwnerLocation)) (.y (Variables|SplineFollowerComponent|GetVirtualOwnerLocation)) (.z (Class|SplineComponent|GetLocationatSplineInputKey (Variables|SplineFollowerComponent|GetCurrentSpline) (LocalVariables|GetClosestKey) "World"))))
                  (if (or (Utilities|Enum|Equal(Enum) AttachToSplineType "NewEnumerator0") (Utilities|Enum|Equal(Enum) AttachToSplineType "NewEnumerator6"))
                    (bind _output_get_4 (LocalVariables|SetStartInputKey (LocalVariables|GetClosestKey)))
                    (Variables|SplineFollowerComponent|SetLastClosestInputKey _output_get_4)
                    (else
                      (bind _output_get_5 (LocalVariables|SetStartInputKey 0.0))
                      (Variables|SplineFollowerComponent|SetLastClosestInputKey _output_get_5))))
                (:then_1
                  (Variables|SplineFollowerComponent|SetCurrentDistanceAlongSpline (Class|SplineComponent|GetDistanceAlongSplineatSplineInputKey (Variables|SplineFollowerComponent|GetCurrentSpline) (LocalVariables|GetStartInputKey)))
                  (if (or (Utilities|Enum|Equal(Enum) AttachToSplineType "NewEnumerator0") (Utilities|Enum|Equal(Enum) AttachToSplineType "NewEnumerator1"))
                    (SplineFollowrComponent|Protected|PlaceOwneratLocation (SplineFollowrComponent|Public|GetOwnerSplineTargetLoc))
                    (else
                      (Variables|SplineFollowerComponent|SetbMovingToStartPoint true))))
                (:then_2
                  (Default|CallOnAttachedtoSpline self (Variables|SplineFollowerComponent|GetCurrentSpline))
                  (if (Utilities|IsValidInterface (Variables|SplineFollowerComponent|GetSplineInterface))
                    (Default|ActorStartedFollowingSpline (Variables|SplineFollowerComponent|GetSplineInterface) (Components|GetOwner) self)))))))))))

(fn SetMoveTarget
  (params (SplineTarget :type Spline%20Target%20Struct%20Structure%20%28by%20ref%29))
  (bind _currentspline (Variables|SplineFollowerComponent|GetCurrentSpline))
  (if (Variables|SplineFollowerComponent|GetbIsLocked)
    (return)
    (else
      (Variables|SplineFollowerComponent|SetSplineTargetType (.MoveTarget (Utilities|Struct|BreakSplineTargetStruct SplineTarget)))
      (Utilities|FlowControl|Sequence
        (:then_0
          (switch Utilities|FlowControl|Switch|SwitchonESplineMoveTargetType (Variables|SplineFollowerComponent|GetSplineTargetType)
            (:NewEnumerator0
              (return))
            (:NewEnumerator1
              (Variables|SplineFollowerComponent|SetTargetSplineKey (Utilities|Struct|BreakSplineTargetStruct SplineTarget)))
            (:NewEnumerator2
              (Variables|SplineFollowerComponent|SetTargetSplineKey (Class|SplineComponent|GetInputKeyValueatSplinePoint _currentspline (- (Spline|GetNumberOfSplinePoints _currentspline) 1))))
            (:NewEnumerator4
              (Variables|SplineFollowerComponent|SetTargetSplineKey (Class|SplineComponent|GetInputKeyValueatSplinePoint (Variables|SplineFollowerComponent|GetCurrentSpline))))))
        (:then_1
          (Variables|SplineFollowerComponent|SetTargetSplineDistance (Class|SplineComponent|GetDistanceAlongSplineatSplineInputKey (Variables|SplineFollowerComponent|GetCurrentSpline) (Variables|SplineFollowerComponent|GetTargetSplineKey)))
          (Components|Tick|SetComponentTickEnabled true))))))

(fn SetupCollisionInfo
  (Utilities|FlowControl|Sequence
    (:then_0
      (bind _asprimitive_component (Utilities|Casting|CastToPrimitiveComponent (Variables|/Script/Engine.Actor|GetRootComponent (Components|GetOwner)))
        (:then
          (LocalVariables|SetPrimitiveComponent _asprimitive_component))
        (:CastFailed
          (LocalVariables|SetPrimitiveComponent (Actor|GetComponentbyClass (Components|GetOwner) "/Script/Engine.PrimitiveComponent")))))
    (:then_1
      (Utilities|IsValid (LocalVariables|GetPrimitiveComponent)
        (:Is%20Valid
          (Variables|SplineFollowerComponent|CollisionSettings|SetCollisionProfile (Collision|GetCollisionProfileName (LocalVariables|GetPrimitiveComponent)))
          (Variables|SplineFollowerComponent|CollisionSettings|SetCollisionRadius (Math|Float|Max(Float) (.X (Math|Vector|BreakVector (.BoxExtent (Collision|GetComponentBounds (LocalVariables|GetPrimitiveComponent))))) (.Y (Math|Vector|BreakVector (.BoxExtent (Collision|GetComponentBounds (LocalVariables|GetPrimitiveComponent)))))))
          (Variables|SplineFollowerComponent|CollisionSettings|SetCollisionHalfHeight (.Z (Math|Vector|BreakVector (.BoxExtent (Collision|GetComponentBounds (LocalVariables|GetPrimitiveComponent)))))))
        (:Is%20Not%20Valid
          (Variables|SplineFollowerComponent|CollisionSettings|SetCollisionProfile (Variables|SplineFollowerComponent|CollisionSettings|GetFallbackCollisionProfileName))
          (Variables|SplineFollowerComponent|CollisionSettings|SetCollisionRadius (Variables|SplineFollowerComponent|CollisionSettings|GetFallbackCollisionRadius))
          (Variables|SplineFollowerComponent|CollisionSettings|SetCollisionHalfHeight (Variables|SplineFollowerComponent|CollisionSettings|GetFallbackCollisionHalfHeight)))))))

(fn MoveOwnerTowardsSplineTarget
  (params (DeltaTime :type Float%20%28double-precision%29))
  (LocalVariables|SetSplineTargetLoc (SplineFollowrComponent|Public|GetOwnerSplineTargetLoc))
  (Utilities|FlowControl|Sequence
    (:then_0
      (switch Utilities|FlowControl|Switch|SwitchonESplineFollowInterpType (Variables|SplineFollowerComponent|MovementStyle|GetLocationInterpType)
        (:NewEnumerator0
          (LocalVariables|SetDesiredLoc (LocalVariables|GetSplineTargetLoc))
          (LocalVariables|SetbFinishedMoving true))
        (:NewEnumerator1
          (bind (_desiredloc _bfinishedmoving) (SplineFollowrComponent|Protected|MoveTowardsTargetLoc (LocalVariables|GetSplineTargetLoc) DeltaTime))
          (LocalVariables|SetDesiredLoc _desiredloc)
          (LocalVariables|SetbFinishedMoving _bfinishedmoving))
        (:NewEnumerator5
          (bind (_desiredloc_2 _bfinishedmoving_2) (SplineFollowrComponent|Protected|InterpTowardsTargetLoc (LocalVariables|GetSplineTargetLoc) DeltaTime))
          (LocalVariables|SetDesiredLoc _desiredloc_2)
          (LocalVariables|SetbFinishedMoving _bfinishedmoving_2))))
    (:then_1
      (SplineFollowrComponent|Protected|PlaceOwneratLocation (LocalVariables|GetDesiredLoc)))
    (:then_2
      (return (LocalVariables|GetbFinishedMoving)))))

(fn MoveTowardsTargetLoc
  (params (TargetLoc :type Vector) (DeltaTime :type Float%20%28double-precision%29))
  (Variables|SplineFollowerComponent|MovementStyle|MoveToTarget|SetCurrentMovementSpeed (Math|Interpolation|FInterptoConstant (Variables|SplineFollowerComponent|MovementStyle|MoveToTarget|GetCurrentMovementSpeed) (Variables|SplineFollowerComponent|MovementStyle|MoveToTarget|GetMoveToTargetMaxSpeed) DeltaTime (Variables|SplineFollowerComponent|MovementStyle|MoveToTarget|GetMoveToTargetAcceleration)))
  (LocalVariables|SetDistanceToTarget (Math|Vector|VectorLength (- (Variables|SplineFollowerComponent|GetVirtualOwnerLocation) TargetLoc)))
  (bind _output_get (LocalVariables|SetNewLoc (Math|Interpolation|VInterptoConstant (Variables|SplineFollowerComponent|GetVirtualOwnerLocation) TargetLoc DeltaTime (select (Variables|SplineFollowerComponent|GetbMovingToStartPoint) (Variables|SplineFollowerComponent|MovementStyle|MoveToTarget|GetCurrentMovementSpeed) (Math|Float|Min(Float) (Variables|SplineFollowerComponent|MovementStyle|MoveToTarget|GetCurrentMovementSpeed) (Math|Float|MapRangeClamped (LocalVariables|GetDistanceToTarget) (Variables|SplineFollowerComponent|MovementStyle|MoveToTarget|GetMoveToTargetSlowDownToEndDistance) 0.0 (Variables|SplineFollowerComponent|MovementStyle|MoveToTarget|GetMoveToTargetMaxSpeed) (Variables|SplineFollowerComponent|MovementStyle|MoveToTarget|GetMoveToTargetSlowingDownMinSpeed)))))))
  (return _output_get (== (Math|Vector|VectorLengthSquared (- TargetLoc (LocalVariables|GetNewLoc))) (LocalVariables|GetDistanceToTarget))))

(fn InterpTowardsTargetLoc
  (params (TargetLoc :type Vector) (DeltaTime :type Float%20%28single-precision%29))
  (LocalVariables|SetNewLoc (Math|Interpolation|VInterpTo (Variables|SplineFollowerComponent|GetVirtualOwnerLocation) TargetLoc DeltaTime (Variables|SplineFollowerComponent|MovementStyle|InterpToTarget|GetLocationInterpSpeed)))
  (return (LocalVariables|GetNewLoc) (Utilities|Operators|EqualEqual (LocalVariables|GetNewLoc) TargetLoc 0.1)))

(fn CalculateEndOwnerPosition
  (params (DesiredLocation :type Vector))
  (return (select (Variables|SplineFollowerComponent|GetOffsetOwnerUpByCapsuleHeight) (+ DesiredLocation (Math|Vector|MakeVector 0.0 0.0 (Variables|SplineFollowerComponent|CollisionSettings|GetCollisionHalfHeight))) DesiredLocation)))

(fn MoveSplineTarget
  (params (DeltaTime :type Float%20%28double-precision%29))
  (if (!= (Variables|SplineFollowerComponent|GetCurrentDistanceAlongSpline) (Variables|SplineFollowerComponent|GetTargetSplineDistance))
    (Utilities|IsValid (Variables|SplineFollowerComponent|GetCurrentSpline)
      (:Is%20Valid
        (Variables|SplineFollowerComponent|SetCurrentDistanceAlongSpline (Math|Interpolation|FInterptoConstant (Variables|SplineFollowerComponent|GetCurrentDistanceAlongSpline) (Variables|SplineFollowerComponent|GetTargetSplineDistance) DeltaTime (Variables|SplineFollowerComponent|GetSplineTargetConstantInterpSpeed)))
        (if (== (Variables|SplineFollowerComponent|GetCurrentDistanceAlongSpline) (Variables|SplineFollowerComponent|GetTargetSplineDistance))
          (Default|CallOnSplineTargetFinishedMove self (Components|GetOwner) (Variables|SplineFollowerComponent|GetCurrentSpline) (Variables|SplineFollowerComponent|GetTargetSplineDistance) (Variables|SplineFollowerComponent|GetTargetSplineKey) (Variables|SplineFollowerComponent|GetSplineTargetType))
          (Variables|SplineFollowerComponent|SetSplineTargetType "NewEnumerator0")
          (return true)
          (else
            (return false)))))))

(fn GetOwnerSplineTargetLoc
  (return (Math|Transform|TransformLocation (Spline|GetTransformatDistanceAlongSpline (Variables|SplineFollowerComponent|GetCurrentSpline) (Variables|SplineFollowerComponent|GetCurrentDistanceAlongSpline) "World" false) (Variables|SplineFollowerComponent|GetSplineFollowOffset))))

(fn PlaceOwneratLocation
  (params (InLoc :type Vector))
  (Variables|SplineFollowerComponent|SetVirtualOwnerLocation InLoc)
  (Utilities|FlowControl|Sequence
    (:then_0
      (bind _ownerlocation (SplineFollowrComponent|Public|CalculateOwnerLocationforDesiredLocation InLoc))
      (Transformation|SetActorLocation (Components|GetOwner) _ownerlocation (Variables|SplineFollowerComponent|GetSweepMovement) false))
    (:then_1
      (LocalVariables|SetClosestInputKey (Class|SplineComponent|FindInputKeyClosesttoWorldLocation (Variables|SplineFollowerComponent|GetCurrentSpline) InLoc))
      (SplineFollowrComponent|Protected|CheckforNotifiesBetweenSplineKeys (Variables|SplineFollowerComponent|GetLastClosestInputKey) (LocalVariables|GetClosestInputKey)))
    (:then_2
      (Variables|SplineFollowerComponent|SetLastClosestInputKey (LocalVariables|GetClosestInputKey)))
    (:then_3
      (if (Math|Boolean|ORBoolean (Variables|SplineFollowerComponent|GetbUseSplineYaw) (Variables|SplineFollowerComponent|GetbUseSplinePitch) (Variables|SplineFollowerComponent|GetbUseSplineRoll))
        (LocalVariables|SetSplineRot (Class|SplineComponent|GetRotationatSplineInputKey (Variables|SplineFollowerComponent|GetCurrentSpline) (LocalVariables|GetClosestInputKey) "World"))
        (LocalVariables|SetOwnerRot (Transformation|GetActorRotation (Components|GetOwner)))
        (LocalVariables|SetTargetRotation (Math|Rotator|MakeRotator (select (Variables|SplineFollowerComponent|GetbUseSplineRoll) (.roll (LocalVariables|GetSplineRot)) (.roll (LocalVariables|GetOwnerRot))) (select (Variables|SplineFollowerComponent|GetbUseSplinePitch) (.pitch (LocalVariables|GetSplineRot)) (.pitch (LocalVariables|GetOwnerRot))) (select (Variables|SplineFollowerComponent|GetbUseSplineYaw) (.yaw (LocalVariables|GetSplineRot)) (.yaw (LocalVariables|GetOwnerRot)))))
        (Transformation|SetActorRotation (Components|GetOwner) (Utilities|Select :Index (Variables|SplineFollowerComponent|MovementStyle|GetRotationInterpType) :NewEnumerator0 (LocalVariables|GetTargetRotation) :NewEnumerator1 (Class|KismetMathLibrary|RInterptoConstant (Transformation|GetActorRotation (Components|GetOwner)) (LocalVariables|GetTargetRotation) (Utilities|Time|GetWorldDeltaSeconds) (Variables|SplineFollowerComponent|MovementStyle|InterpToTarget|GetRotationInterpSpeed)) :NewEnumerator5 (Math|Interpolation|RInterpTo (Transformation|GetActorRotation (Components|GetOwner)) (LocalVariables|GetTargetRotation) (Utilities|Time|GetWorldDeltaSeconds) (Variables|SplineFollowerComponent|MovementStyle|InterpToTarget|GetRotationInterpSpeed))))))))

(fn IsMovingAlongSpline
  (return (and (Utilities|IsValid (Variables|SplineFollowerComponent|GetCurrentSpline)) (Utilities|Enum|NotEqual(Enum) (Variables|SplineFollowerComponent|GetSplineTargetType) "NewEnumerator0")) (Variables|SplineFollowerComponent|GetbIsPausedOnSpline)))

(fn CheckforNotifiesBetweenSplineKeys
  (params (SplineKeyA :type Float%20%28double-precision%29) (SplineKeyB :type Float%20%28double-precision%29))
  (if (!= SplineKeyA SplineKeyB)
    (for _array_element (Variables|SplineFollowerComponent|GetCurrentSplineNotifies)
      (bind _output_get (LocalVariables|SetTempNotify _array_element))
      (bind _output_get_2 (LocalVariables|SetNotifyNormalisedPoint (Math|Float|MapRangeUnclamped (Utilities|Struct|BreakSplineNotifyStruct _output_get) SplineKeyA SplineKeyB 0.0 1.0)))
      (if (and (>= _output_get_2 0.0) (<= _output_get_2 1.0))
        (if (Utilities|IsValidInterface (Variables|SplineFollowerComponent|GetSplineInterface))
          (Default|FollowerPassedNotify (Variables|SplineFollowerComponent|GetSplineInterface) (Components|GetOwner) self (LocalVariables|GetTempNotify)))))
    (else
      (return))))

(fn DebugSplineFollower
  (if (and (not (Class|KismetSystemLibrary|IsPackagedforDistribution)) (Variables|SplineFollowerComponent|GetbInDebugMode))
    (bind _output_get (LocalVariables|SetCurrentWorldLoc (Spline|GetLocationatDistanceAlongSpline (Variables|SplineFollowerComponent|GetCurrentSpline) (Variables|SplineFollowerComponent|GetCurrentDistanceAlongSpline) "World")))
    (Rendering|Debug|DrawDebugSphere _output_get 2e+01 12 "(R=0.000000,G=1.000000,B=0.169006,A=1.000000)" 0.0)
    (Rendering|Debug|DrawDebugString (LocalVariables|GetCurrentWorldLoc) "Current spline location" (Components|GetOwner) "(R=0.000000,G=1.000000,B=0.146768,A=1.000000)")
    (bind _output_get_2 (LocalVariables|SetTargetWorldLoc (Spline|GetLocationatDistanceAlongSpline (Variables|SplineFollowerComponent|GetCurrentSpline) (Variables|SplineFollowerComponent|GetTargetSplineDistance) "World")))
    (Rendering|Debug|DrawDebugSphere _output_get_2 2e+01 12 "(R=1.000000,G=0.000000,B=0.041855,A=1.000000)" 0.0)
    (Rendering|Debug|DrawDebugString (LocalVariables|GetTargetWorldLoc) "Current spline location" (Components|GetOwner) "(R=1.000000,G=0.000000,B=0.065008,A=1.000000)")
    (Development|PrintString (Utilities|String|Append "Current spline key: " (Utilities|String|ToString(Float) (Variables|SplineFollowerComponent|GetLastClosestInputKey))) true true "(R=0.000000,G=1.000000,B=0.207774,A=1.000000)" 5.0 "ClosestSplineInput")))

(fn SphereTraceforFloor
  (params (TargetLoc :type Vector) (ActorsToIgnore :type Array%20of%20Actor%20Object%20References) (Retries :type Integer))
  (LocalVariables|SetTraceStart (+ TargetLoc (Math|Vector|MakeVector 0.0 0.0 (Variables|SplineFollowerComponent|GetTraceOffsetHeight))))
  (bind (_outhit _returnvalue) (Class|KismetSystemLibrary|SphereTraceSinglebyProfile (LocalVariables|GetTraceStart) (- TargetLoc (Math|Vector|MakeVector 0.0 0.0 (Variables|SplineFollowerComponent|GetTraceOffsetHeight))) (Variables|SplineFollowerComponent|CollisionSettings|GetCollisionRadius) (Variables|SplineFollowerComponent|CollisionSettings|GetCollisionProfile) false ActorsToIgnore "None" true))
  (if (and (.bInitialOverlap (Collision|BreakHitResult _outhit)) (> Retries 0))
    (Utilities|Array|Add ActorsToIgnore (.HitActor (Collision|BreakHitResult _outhit)))
    (bind (_outhit_2 _returnvalue_2) (SplineFollowrComponent|Protected|SphereTraceforFloor TargetLoc ActorsToIgnore (- Retries 1)))
    (return _outhit_2 _returnvalue_2)
    (else
      (return _outhit _returnvalue))))

(fn PauseSplineMovement
  (Variables|SplineFollowerComponent|SetbIsPausedOnSpline true))

(fn ResumeSplineMovement
  (Variables|SplineFollowerComponent|SetbIsPausedOnSpline false))

(fn CalculateOwnerLocationforDesiredLocation
  (params (DesiredLocation :type Vector))
  (if (Variables|SplineFollowerComponent|GetTraceForFloor)
    (bind _output_get (LocalVariables|SetIgnoreActorArray (Actor|GetAttachedActors (Components|GetOwner) true true)))
    (Utilities|Array|Add _output_get (Components|GetOwner))
    (bind (_outhit _returnvalue) (SplineFollowrComponent|Protected|SphereTraceforFloor DesiredLocation (LocalVariables|GetIgnoreActorArray) 3))
    (if _returnvalue
      (return (+ (.Location (Collision|BreakHitResult _outhit)) (Math|Vector|MakeVector 0.0 0.0 (- (Variables|SplineFollowerComponent|CollisionSettings|GetCollisionHalfHeight) (Variables|SplineFollowerComponent|CollisionSettings|GetCollisionRadius)))))
      (else
        (return (SplineFollowrComponent|Protected|CalculateEndOwnerPosition DesiredLocation))))
    (else
      (return (SplineFollowrComponent|Protected|CalculateEndOwnerPosition DesiredLocation)))))

(fn ClearSplineTarget)

(fn LockSplineFollowLogic
  (Variables|SplineFollowerComponent|SetSplineTargetType "NewEnumerator0")
  (Variables|SplineFollowerComponent|SetbIsLocked true)
  (Components|Tick|SetComponentTickEnabled false))

(fn GetIsinDebug
  (return (Variables|SplineFollowerComponent|GetbInDebugMode)))