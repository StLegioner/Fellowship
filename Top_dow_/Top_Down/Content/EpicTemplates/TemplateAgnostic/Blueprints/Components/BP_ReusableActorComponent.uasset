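; BP_ReusableActorComponent lets its owning actor be pooled and reused through an actor reuse manager.
; One tick after BeginPlay it requests registration with the manager unless BindReuseManager has already bound a ready-for-reuse callback and flagged it managed.
; It tracks readiness and broadcasts dispatchers when ready or reset.
; A deferred destroy request fires a destroy-self dispatcher immediately if already ready, otherwise when next marked ready.
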(event Custom|CheckForReuseManagement
  (if (not (Variables|Default|GetbReuseIsManaged))
    (bind _actorreusemanager (CallFunction|GetActorReuseManager))
    (Default|RequestRegistration _actorreusemanager self (Components|GetOwner))))

(event EventBeginPlay
  (Class|KismetSystemLibrary|SetTimerforNextTickDelegate (delegate Custom|CheckForReuseManagement)))

(fn GetIsReadyforReuse
  (return (Variables|Default|GetbReadyForReuse)))

(fn MarkReadyforReuse
  (Variables|Default|SetbReadyForReuse true)
  (Default|CallOnReadyforReuse self (Components|GetOwner))
  (if (Variables|Default|GetbRequestDestroyOnNextReadyForReuse)
    (Default|CallOnRequestDestroySelf)))

(fn ResetActor
  (Default|CallOnResetRequested self (Components|GetOwner))
  (Variables|Default|SetbReadyForReuse false))

(fn RequestDestroyonNextReadyforReuse
  (Variables|Default|SetbRequestDestroyOnNextReadyForReuse true)
  (if (Variables|Default|GetbReadyForReuse)
    (Default|CallOnRequestDestroySelf)))

(fn BindReuseManager
  (params (ReadyForReuseCallback :type Delegate%20%28by%20ref%29))
  (EventDispatchers|BindEventtoOnReadyforReuse ReadyForReuseCallback)
  (Variables|Default|SetbReuseIsManaged true))