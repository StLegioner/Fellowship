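; Actor component that applies damage to damageable actors touching its registered primitive components, on contact and repeatedly on a looping timer.
; Begin and end overlaps maintain the target list and timer, skipping same-team actors via BPI_TeamParticipant.
; Registering a primitive also damages existing overlaps, without the team check or timer start, and unregistering prunes targets.
; The owner's BP_ReusableActorComponent clears targets and timer when ready for reuse.
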(event Custom|RegisterTouchComponent
  (params (PrimitiveComponent :type Primitive%20Component%20Object%20Reference%20%28by%20ref%29))
  ;[1 1 1] Register/Unregister touch component
  (bind _returnvalue (Utilities|Array|AddUnique (Variables|Default|GetTouchComponents) PrimitiveComponent))
  (if (>= _returnvalue 0)
    (Collision|BindEventtoOnComponentBeginOverlap PrimitiveComponent (EventDispatchers|CreateEvent :!event Custom|BeginTouchComponentOverlap))
    (Collision|BindEventtoOnComponentEndOverlap PrimitiveComponent (EventDispatchers|CreateEvent :!event Custom|EndTouchComponentOverlap))
    (CallFunction|CheckforExistingOverlaps PrimitiveComponent)))

(event Custom|ParentActorReadyForReuse
  (params (Caller :type BP%20Reusable%20Actor%20Component%20Object%20Reference) (ActorForReuse :type Actor%20Object%20Reference))
  ;[1 1 1] Parent actor reusable actor component binds
  (Utilities|Time|ClearandInvalidateTimerbyHandle (Variables|Default|GetDamageTimer))
  (Utilities|Array|Clear (Variables|Default|GetDamageTargets)))

(event Custom|DamageAllAttackTargets
  ;[1 1 1] Begin/End overlaps
  (for _array_element (Variables|Default|GetDamageTargets)
    (CallFunction|DamageTarget _array_element)))

(event Custom|UnregisterTouchComponent
  (params (PrimitiveComponent :type Primitive%20Component%20Object%20Reference%20%28by%20ref%29))
  ;[1 1 1] Register/Unregister touch component
  (bind _returnvalue (Utilities|Array|RemoveItem (Variables|Default|GetTouchComponents) PrimitiveComponent))
  (if _returnvalue
    (Collision|UnbindEventfromOnComponentBeginOverlap PrimitiveComponent (EventDispatchers|CreateEvent :!event Custom|BeginTouchComponentOverlap))
    (Collision|UnbindEventfromOnComponentEndOverlap PrimitiveComponent (EventDispatchers|CreateEvent :!event Custom|EndTouchComponentOverlap))
    (CallFunction|RemoveNoLongerOverlappedInteracts)))

(event Custom|BeginTouchComponentOverlap
  (params (OverlappedComponent :type Primitive%20Component%20Object%20Reference) (OtherActor :type Actor%20Object%20Reference) (OtherComp :type Primitive%20Component%20Object%20Reference) (OtherBodyIndex :type Integer) (bFromSweep :type Boolean) (SweepResult :type Hit%20Result%20Structure%20%28by%20ref%29))
  ;[1 1 1] Begin/End overlaps
  (bind _damageable (CallFunction|IsActorValidDamageRecipient OtherActor))
  (if (Utilities|IsValidInterface _damageable)
    (Utilities|Array|Add (Variables|Default|GetDamageTargets) (Utilities|Struct|MakeAttackTargetStruct OtherActor _damageable))
    (CallFunction|DamageTarget (Utilities|Struct|MakeAttackTargetStruct OtherActor _damageable))
    (if (not (Utilities|Time|IsValidTimerHandle (Variables|Default|GetDamageTimer)))
      (bind _returnvalue (Utilities|Time|SetTimerbyEvent (delegate Custom|DamageAllAttackTargets) (Variables|Default|GetDamageFrequency) true))
      (Variables|Default|SetDamageTimer _returnvalue))))

(event Custom|EndTouchComponentOverlap
  (params (OverlappedComponent :type Primitive%20Component%20Object%20Reference) (OtherActor :type Actor%20Object%20Reference) (OtherComp :type Primitive%20Component%20Object%20Reference) (OtherBodyIndex :type Integer))
  ;[1 1 1] Begin/End overlaps
  (bind _targetremoved (CallFunction|TryRemoveActorfromTargets OtherActor))
  (if _targetremoved
    (if (<= (Utilities|Array|Length (Variables|Default|GetDamageTargets)) 0)
      (Utilities|Time|ClearandInvalidateTimerbyHandle (Variables|Default|GetDamageTimer)))))

(event EventBeginPlay
  ;[1 1 1] BeginPlay
  (CallFunction|SetupParentActorConnections))

(fn IsActorValidDamageRecipient
  (params (InputPin :type Actor%20Object%20Reference))
  (Utilities|FlowControl|Sequence
    (:then_0
      (if (Utilities|IsValidInterface (Variables|Default|GetParentTeamInterface))
        (bind _interfaceimplementingobject (CallFunction|SearchActorforInterface InputPin "/Game/EpicTemplates/TemplateAgnostic/Blueprints/Interfaces/BPI_TeamParticipant.BPI_TeamParticipant_C" false))
        (Utilities|IsValid _interfaceimplementingobject
          (:Is%20Valid
            (bind _team (Class|BPITeamParticipant|GetTeam(Message) _interfaceimplementingobject))
            (bind _team_2 (Default|GetTeam (Variables|Default|GetParentTeamInterface)))
            (if (Utilities|Enum|Equal(Enum) _team_2 _team)
              (return 0 false))))))
    (:then_1
      (bind _interfaceimplementingobject_2 (CallFunction|SearchActorforInterface InputPin "/Game/EpicTemplates/TemplateAgnostic/Blueprints/Interfaces/BPI_Damageable.BPI_Damageable_C" false))
      (bind _asbpi_damageable (Utilities|Casting|CastToBPI_Damageable _interfaceimplementingobject_2))
      (return _asbpi_damageable true))
    (:then_2
      (return 0 false))))

(fn TryRemoveActorfromTargets
  (params (Actor :type Object%20Object%20Reference))
  (Utilities|FlowControl|Sequence
    (:then_0
      (for (_array_element _array_index) (Variables|Default|GetDamageTargets)
        (LocalVariables|SetTargetIdx _array_index)
        (if (== (Utilities|Struct|BreakAttackTargetStruct _array_element) Actor)
          (Utilities|Array|RemoveIndex (Variables|Default|GetDamageTargets) (LocalVariables|GetTargetIdx))
          (return true))))
    (:then_1
      (return false))))

(fn DamageTarget
  (params (AttackTarget :type Attack%20Target%20Struct%20Structure%20%28by%20ref%29))
  (bind _returnvalue (Components|GetOwner))
  (Default|ApplyDamage (Utilities|Struct|BreakAttackTargetStruct AttackTarget) (Utilities|Struct|MakeDamageStruct (Variables|Default|GetDamage) _returnvalue _returnvalue (Transformation|GetActorLocation (Components|GetOwner)) (Math|Vector|Normalize (- (Transformation|GetActorLocation (Utilities|Struct|BreakAttackTargetStruct AttackTarget)) (Transformation|GetActorLocation (Components|GetOwner)))))))

(fn SetupParentActorConnections
  (Utilities|FlowControl|Sequence
    (:then_0
      (bind _interfaceimplementingobject (CallFunction|SearchActorforInterface (Components|GetOwner) "/Game/EpicTemplates/TemplateAgnostic/Blueprints/Interfaces/BPI_TeamParticipant.BPI_TeamParticipant_C" false))
      (bind _asbpi_team_participant (Utilities|Casting|CastToBPI_TeamParticipant _interfaceimplementingobject))
      (Variables|Default|SetParentTeamInterface _asbpi_team_participant))
    (:then_1
      (bind _output_get (LocalVariables|SetReusableActorComponent (Actor|GetComponentbyClass (Components|GetOwner) "/Game/EpicTemplates/TemplateAgnostic/Blueprints/Components/BP_ReusableActorComponent.BP_ReusableActorComponent_C")))
      (Utilities|IsValid _output_get
        (:Is%20Valid
          (EventDispatchers|BindEventtoOnReadyforReuse (LocalVariables|GetReusableActorComponent) (EventDispatchers|CreateEvent :!event Custom|ParentActorReadyForReuse)))))))

(fn GetInteractionDetectionObjectTypeArray
  (return (Utilities|Array|MakeArray "ObjectTypeQuery2" "ObjectTypeQuery3" "ObjectTypeQuery4" "ObjectTypeQuery5" "ObjectTypeQuery8")))

(fn CheckforExistingOverlaps
  (params (OverlapComponent :type Primitive%20Component%20Object%20Reference))
  (bind _outactors (Collision|ComponentOverlapActors OverlapComponent (Transformation|GetWorldTransform OverlapComponent) (Variables|Default|GetTouchObjectTypes) 0 (Utilities|Array|MakeArray (Components|GetOwner))))
  (for _array_element _outactors
    (LocalVariables|SetTempActor _array_element)
    (Utilities|FlowControl|Sequence
      (:then_0
        (LocalVariables|SetNoMatchFound true)
        (bind _array_element_2 (Utilities|Array|ForEachLoopwithBreak (Variables|Default|GetDamageTargets) :!label _label)
          (:LoopBody
            (if (== (.TargetActor (Utilities|Struct|BreakAttackTargetStruct _array_element_2)) (LocalVariables|GetTempActor))
              (LocalVariables|SetNoMatchFound false)
              (goto _label Break)))))
      (:then_1
        (if (LocalVariables|GetNoMatchFound)
          (bind _interfaceimplementingobject (CallFunction|SearchActorforInterface (LocalVariables|GetTempActor) "/Game/EpicTemplates/TemplateAgnostic/Blueprints/Interfaces/BPI_Damageable.BPI_Damageable_C" false))
          (bind _asbpi_damageable (Utilities|Casting|CastToBPI_Damageable _interfaceimplementingobject))
          (Utilities|Array|Add (Variables|Default|GetDamageTargets) (Utilities|Struct|MakeAttackTargetStruct (LocalVariables|GetTempActor) _asbpi_damageable))
          (CallFunction|DamageTarget (Utilities|Struct|MakeAttackTargetStruct (LocalVariables|GetTempActor) _asbpi_damageable)))))))

(fn RemoveNoLongerOverlappedInteracts
  (Utilities|FlowControl|Sequence
    (:then_0
      (bind _output_get (LocalVariables|SetUnoverlappedTargets (Variables|Default|GetDamageTargets)))
      (for (_array_element _array_index) _output_get
        (LocalVariables|SetTempIndex _array_index)
        (LocalVariables|SetTempActor (Utilities|Struct|BreakAttackTargetStruct _array_element))
        (bind _array_element_2 (Utilities|Array|ForEachLoopwithBreak (Variables|Default|GetTouchComponents) :!label _label)
          (:LoopBody
            (if (>= (Utilities|Array|FindItem (Collision|GetOverlappingActors _array_element_2 0 :!class /Script/Engine.PrimitiveComponent) (LocalVariables|GetTempActor)) 0)
              (Utilities|Array|RemoveIndex (LocalVariables|GetUnoverlappedTargets) (LocalVariables|GetTempIndex))
              (goto _label Break))))))
    (:then_1
      (for _array_element_3 (LocalVariables|GetUnoverlappedTargets)
        (LocalVariables|SetTempActor (Utilities|Struct|BreakAttackTargetStruct _array_element_3))
        (bind (_array_element_4 _array_index_2) (Utilities|Array|ForEachLoopwithBreak (Variables|Default|GetDamageTargets) :!label _label_2)
          (:LoopBody
            (LocalVariables|SetTempIndex _array_index_2)
            (if (== (Utilities|Struct|BreakAttackTargetStruct _array_element_4) (LocalVariables|GetTempActor))
              (Utilities|Array|RemoveIndex (Variables|Default|GetDamageTargets) (LocalVariables|GetTempIndex))
              (goto _label_2 Break))))))))