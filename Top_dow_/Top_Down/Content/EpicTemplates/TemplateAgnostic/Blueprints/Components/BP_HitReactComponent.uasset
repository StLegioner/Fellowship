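; Actor component that plays hit feedback when damaged: a temporary material swap on registered meshes, plus a particle and sound.
; Can auto-bind to the owner's BP_HealthComponent, reacting whenever damage changes health.
; Registration caches default materials per slot, and a timer restores them.
; Assets load asynchronously, with the material applied only while that timer runs and the particle oriented against the damage direction.
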(event Custom|OwnerTookDamage
  (params (Caller :type BP%20Health%20Component%20Object%20Reference) (OldHealth :type Float%20%28double-precision%29) (NewHealth :type Float%20%28double-precision%29) (SpecialDamageName :type Name) (DamageStruct :type Damage%20Struct%20Structure%20%28by%20ref%29))
  ;[1 1 1] Owner took dmaage
  (if (!= OldHealth NewHealth)
    (CallFunction|PerformHitReact DamageStruct)))

(event Custom|RegisterReactMesh
  (params (MeshComponent :type Mesh%20Component%20Object%20Reference%20%28by%20ref%29) (MaterialSlots :type Array%20of%20Integers) (bAddAllMaterialSlots :type Boolean))
  ;[1 1 1] Add/Remove React Mesh
  (CallFunction|HandleAddReactMesh MeshComponent MaterialSlots bAddAllMaterialSlots))

(event Custom|UnregisterReactMesh
  (params (MeshComponent :type Mesh%20Component%20Object%20Reference))
  ;[1 1 1] Add/Remove React Mesh
  (Utilities|Map|Remove (Variables|HitReactComponent|GetCurrentReactMeshes) MeshComponent))

(event Custom|PerformHitReact
  (params (DamageStruct :type Damage%20Struct%20Structure%20%28by%20ref%29))
  (bind (_damagelocation _damagedirection) (Utilities|Struct|BreakDamageStruct DamageStruct))
  ;[1 1 1] Hit react
  (Utilities|FlowControl|Sequence
    (:then_0
      (bind _returnvalue (Utilities|Time|SetTimerbyEvent (EventDispatchers|CreateEvent :!event Custom|FinishHitReact) (Variables|HitReactComponent|GetHitReactTime)))
      (Variables|HitReactComponent|SetHitReactTimer _returnvalue))
    (:then_1
      (bind _object (Utilities|AsyncLoadAsset (Variables|HitReactComponent|GetHitReactMaterial))
        (:Completed
          (if (Utilities|Time|IsTimerActivebyHandle (Variables|HitReactComponent|GetHitReactTimer))
            (bind _asmaterial_interface (Utilities|Casting|CastToMaterialInterface _object))
            (CallFunction|UpdateReactMeshestoHitReactMaterial _asmaterial_interface)))))
    (:then_2
      (Utilities|PlaySoftNiagaraParticleAsyncatLocation (Variables|HitReactComponent|GetHitReactParticle) _damagelocation (Math|Rotator|MakeRotfromXZ (* _damagedirection -1.0) (Math|Vector|MakeVector 0.0 0.0 1.0))
        (:Immedate
          (Utilities|PlaySoftSoundAsyncatLocation (Variables|HitReactComponent|GetHitReactSound) _damagelocation))))))

(event Custom|FinishHitReact
  ;[1 1 1] React Finished
  (CallFunction|UpdateReactMeshestoDefaults)
  (Default|CallOnHitReactFinished self))

(event EventBeginPlay
  ;[1 1 1] Begin Play
  (CallFunction|BindtoHealthEvents))

(fn IsCurrentlyHitReacting
  (return (Utilities|Time|IsTimerActivebyHandle (Variables|HitReactComponent|GetHitReactTimer))))

(fn HandleAddReactMesh
  (params (MeshComponent :type Mesh%20Component%20Object%20Reference) (MaterialSlots :type Array%20of%20Integers) (bAddAllMaterialSlots :type Boolean))
  (Utilities|FlowControl|Sequence
    (:then_0
      (if bAddAllMaterialSlots
        (Utilities|Array|Resize MaterialSlots (Utilities|Array|Length (Rendering|Material|GetMaterials MeshComponent)))
        (for (_ _array_index) MaterialSlots
          (Utilities|Array|SetArrayElem MaterialSlots _array_index _array_index))))
    (:then_1
      (Utilities|Struct|SetmembersinHitReactMeshTargetStruct (LocalVariables|GetNewEntry) MeshComponent MaterialSlots)
      (Utilities|Array|Resize (Utilities|Struct|BreakHitReactMeshTargetStruct (LocalVariables|GetNewEntry)) (Utilities|Array|Length MaterialSlots))
      (for _array_element MaterialSlots
        (Utilities|Array|SetArrayElem (Utilities|Struct|BreakHitReactMeshTargetStruct (LocalVariables|GetNewEntry)) _array_element (Rendering|Material|GetMaterial MeshComponent _array_element) true)))
    (:then_2
      (Utilities|Map|Add (Variables|HitReactComponent|GetCurrentReactMeshes) MeshComponent (LocalVariables|GetNewEntry))
      (bind _values (Utilities|Map|Values (Variables|HitReactComponent|GetCurrentReactMeshes)))
      (Variables|HitReactComponent|SetReactStructs _values))))

(fn BindtoHealthEvents
  (if (Variables|HitReactComponent|GetbAutoBindToParentHealthComponent)
    (bind _output_get (LocalVariables|SetOwnerHealthComponent (Actor|GetComponentbyClass (Components|GetOwner) "/Game/EpicTemplates/TemplateAgnostic/Blueprints/Components/BP_HealthComponent.BP_HealthComponent_C")))
    (Utilities|IsValid _output_get
      (:Is%20Valid
        (EventDispatchers|BindEventtoOnTookDamage (LocalVariables|GetOwnerHealthComponent) (EventDispatchers|CreateEvent :!event Custom|OwnerTookDamage))))))

(fn UpdateReactMeshestoHitReactMaterial
  (params (ReactMaterial :type Material%20Interface%20Object%20Reference))
  (for _array_element (Variables|HitReactComponent|GetReactStructs)
    (LocalVariables|SetTempMesh (.MeshComponent (Utilities|Struct|BreakHitReactMeshTargetStruct _array_element)))
    (for _array_element_2 (.MaterialSlots (Utilities|Struct|BreakHitReactMeshTargetStruct _array_element))
      (Rendering|Material|SetMaterial (LocalVariables|GetTempMesh) _array_element_2 ReactMaterial))))

(fn UpdateReactMeshestoDefaults
  (for _array_element (Variables|HitReactComponent|GetReactStructs)
    (LocalVariables|SetTempMesh (.MeshComponent (Utilities|Struct|BreakHitReactMeshTargetStruct _array_element)))
    (for (_array_element_2 _array_index) (.MaterialSlots (Utilities|Struct|BreakHitReactMeshTargetStruct _array_element))
      (Rendering|Material|SetMaterial (LocalVariables|GetTempMesh) _array_element_2 (Utilities|Array|Get(acopy) (.DefaultMaterials (Utilities|Struct|BreakHitReactMeshTargetStruct _array_element)) _array_index)))))