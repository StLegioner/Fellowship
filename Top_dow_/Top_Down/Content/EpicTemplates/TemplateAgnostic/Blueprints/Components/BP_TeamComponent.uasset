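; BP_TeamComponent is a component that stores the current team of its owner and announces when it changes.
; It copies InitialTeam into CurrentTeam on BeginPlay, and AssignTeam fires OnTeamChanged only when the new team differs.
; GetTeam returns InitialTeam until a valid GameState has begun play, so early queries do not read an uninitialized CurrentTeam.
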(event EventAssignTeam
  (params (NewTeam :type EGameTeam%20Enum :default "NewEnumerator0"))
  (if (Utilities|Enum|NotEqual(Enum) NewTeam (Variables|TeamComponent|GetCurrentTeam))
    (bind _output_get (Variables|TeamComponent|SetCurrentTeam NewTeam))
    (Default|CallOnTeamChanged self _output_get)))

(event EventBeginPlay
  (Variables|TeamComponent|SetCurrentTeam (Variables|TeamComponent|GetInitialTeam)))

(fn GetTeam
  (bind _returnvalue (Game|GetGameState))
  (Utilities|IsValid _returnvalue
    (:Is%20Valid
      (if (Class|GameStateBase|HasBegunPlay _returnvalue)
        (return (Variables|TeamComponent|GetCurrentTeam))
        (else
          _)))
    (:Is%20Not%20Valid
      _))
  (return (Variables|TeamComponent|GetInitialTeam)))