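; BP_PlayerScoreComponent is a component that keeps a player's current score and exposes add, subtract and read operations.
; Each change takes its value from a score source passed in by the caller.
; Additions apply the source's modifier multipliers in sequence, truncating to an integer after each, while subtractions use the raw value.
; Both then fire a notification carrying the old score, new score, source and modifiers.
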(event EventAddScore
  (params (NewSource :type BPI%20Game%20Score%20Source%20Interface))
  (CallFunction|AddScoreInternal NewSource))

(event EventSubtractScore
  (params (ScoreSource :type BPI%20Game%20Score%20Source%20Interface))
  (CallFunction|SubtractScoreInternal ScoreSource))

(fn AddScoreInternal
  (params (ScoreSource :type BPI%20Game%20Score%20Source%20Interface))
  (bind _scorevalue (Default|GetScoreValue ScoreSource))
  (LocalVariables|SetScoreToAdd _scorevalue)
  (LocalVariables|SetOldScore (Variables|Default|GetCurrentScore))
  (Utilities|FlowControl|Sequence
    (:then_0
      (bind _modifiers (Default|GetModifiers ScoreSource))
      (bind _output_get (LocalVariables|SetModifiers _modifiers))
      (for _array_element _output_get
        (LocalVariables|SetScoreToAdd (Math|Float|Truncate (* (Math|Conversions|ToFloat(Integer) (LocalVariables|GetScoreToAdd)) (.ModifierMultiplier (Utilities|Struct|BreakScoreModifierStruct _array_element)))))))
    (:then_1
      (CallFunction|PlusEqualsInt (Variables|Default|GetCurrentScore) (LocalVariables|GetScoreToAdd))
      (Default|CallOnScoreAdded (LocalVariables|GetOldScore) (Variables|Default|GetCurrentScore) ScoreSource (LocalVariables|GetModifiers)))))

(fn SubtractScoreInternal
  (params (ScoreSource :type BPI%20Game%20Score%20Source%20Interface))
  (bind _scorevalue (Default|GetScoreValue ScoreSource))
  (LocalVariables|SetOldScore (Variables|Default|GetCurrentScore))
  (CallFunction|MinusEqualsInt (Variables|Default|GetCurrentScore) _scorevalue)
  (Default|CallOnScoreSubtracted (LocalVariables|GetOldScore) (Variables|Default|GetCurrentScore) ScoreSource (Utilities|Array|MakeArray)))

(fn GetCurrentScore
  (return (Variables|Default|GetCurrentScore)))