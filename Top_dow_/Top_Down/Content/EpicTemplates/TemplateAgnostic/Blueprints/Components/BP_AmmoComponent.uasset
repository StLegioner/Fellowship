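; Actor component that tracks current and max ammo per ammo type, seeded from start maps on BeginPlay.
; Internal update functions write the maps and fire change events, with unknown types in ammo updates also setting their max.
; TrySpendAmmoOfType supports all-or-nothing or partial spending by spend type, treats negative ammo as infinite, and raises spent, emptied or tried-empty events.
; Getters expose amounts and a display-as-percent flag.
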(event EventUpdateMaxAmmoOfType
  (params (AmmoType :type EAmmoType%20Enum :default "NewEnumerator2") (NewMaxAmmo :type Float%20%28double-precision%29))
  (CallFunction|UpdateMaxAmmoInternal AmmoType NewMaxAmmo))

(event EventUpdateAmmoOfType
  (params (AmmoType :type EAmmoType%20Enum :default "NewEnumerator2") (NewAmmo :type Float%20%28double-precision%29))
  (CallFunction|UpdateAmmoInternal AmmoType NewAmmo))

(event EventBeginPlay
  ;[1 1 1] Begin Play
  (Utilities|FlowControl|Sequence
    (:then_0
      (bind _keys (Utilities|Map|Keys (Variables|Default|GetStartMaxAmmo)))
      (for _array_element _keys
        (CallFunction|UpdateMaxAmmoInternal _array_element (.Value (Utilities|Map|Find (Variables|Default|GetStartMaxAmmo) _array_element)))))
    (:then_1
      (bind _keys_2 (Utilities|Map|Keys (Variables|Default|GetStartAmmo)))
      (for _array_element_2 _keys_2
        (CallFunction|UpdateAmmoInternal _array_element_2 (.Value (Utilities|Map|Find (Variables|Default|GetStartAmmo) _array_element_2)))))))

(fn UpdateMaxAmmoInternal
  (params (AmmoType :type EAmmoType%20Enum :default "NewEnumerator0") (NewMaxAmmo :type Float%20%28double-precision%29))
  (bind _maxammo (Variables|Default|GetMaxAmmo))
  (bind (_value _returnvalue) (Utilities|Map|Find _maxammo AmmoType))
  (LocalVariables|SetOldMaxAmmo _value)
  (if (or (== _returnvalue false) (!= (LocalVariables|GetOldMaxAmmo) NewMaxAmmo))
    (Utilities|Map|Add (Variables|Default|GetMaxAmmo) AmmoType NewMaxAmmo)
    (Default|CallOnMaxAmmoUpdated self AmmoType (LocalVariables|GetOldMaxAmmo) NewMaxAmmo)))

(fn UpdateAmmoInternal
  (params (AmmoType :type EAmmoType%20Enum :default "NewEnumerator0") (NewAmmo :type Float%20%28double-precision%29))
  (bind _currentammo (Variables|Default|GetCurrentAmmo))
  (bind (_value _returnvalue) (Utilities|Map|Find _currentammo AmmoType))
  (LocalVariables|SetOldAmmo _value)
  (LocalVariables|SetFoundAmmoType _returnvalue)
  (Utilities|FlowControl|Sequence
    (:then_0
      (if (not (LocalVariables|GetFoundAmmoType))
        (Utilities|Map|Add (Variables|Default|GetMaxAmmo) AmmoType NewAmmo)
        (Default|CallOnMaxAmmoUpdated self AmmoType 0.0 NewAmmo)))
    (:then_1
      (if (or (not (LocalVariables|GetFoundAmmoType)) (!= (LocalVariables|GetOldAmmo) NewAmmo))
        (Utilities|Map|Add (Variables|Default|GetCurrentAmmo) AmmoType NewAmmo)
        (Default|CallOnAmmoUpdated self AmmoType (LocalVariables|GetOldAmmo) NewAmmo)))))

(fn GetCurrentAmmoOfType
  (params (AmmoType :type EAmmoType%20Enum :default "NewEnumerator2"))
  (bind _currentammo (Variables|Default|GetCurrentAmmo))
  (bind (_value _returnvalue) (Utilities|Map|Find _currentammo AmmoType))
  (if _returnvalue
    (return _value)
    (else
      (return 0.0))))

(fn GetMaxAmmoOfType
  (params (AmmoType :type EAmmoType%20Enum :default "NewEnumerator2"))
  (bind _maxammo (Variables|Default|GetMaxAmmo))
  (bind (_value _returnvalue) (Utilities|Map|Find _maxammo AmmoType))
  (if _returnvalue
    (return _value)
    (else
      (return 0.0))))

(fn IsAmmoPercentage
  (return (Variables|Default|GetbDisplayAmmoAsPercent)))

(fn TrySpendAmmoOfType
  (params (AmmoType :type EAmmoType%20Enum :default "NewEnumerator2") (AmmoToSpend :type Float%20%28double-precision%29) (SpendType :type EAmmoSpendType%20Enum :default "NewEnumerator0"))
  (bind _output_get (LocalVariables|SetOldAmmo (.Value (Utilities|Map|Find (Variables|Default|GetCurrentAmmo) AmmoType))))
  (if (> _output_get 0.0)
    (bind _output_get_2 (LocalVariables|SetSpentAmmo (+ AmmoToSpend (Math|Float|Min(Float) (- (LocalVariables|GetOldAmmo) AmmoToSpend) 0.0))))
    (if (or (== _output_get_2 AmmoToSpend) (Utilities|Enum|Equal(Enum) SpendType "NewEnumerator1"))
      (bind _output_get_3 (LocalVariables|SetNewAmmo (- (LocalVariables|GetOldAmmo) (LocalVariables|GetSpentAmmo))))
      (Utilities|Map|Add (Variables|Default|GetCurrentAmmo) AmmoType _output_get_3)
      (Default|CallOnSpentAmmo self AmmoType (LocalVariables|GetOldAmmo) (LocalVariables|GetNewAmmo))
      (Utilities|FlowControl|Sequence
        (:then_0
          (if (<= (LocalVariables|GetNewAmmo) 0.0)
            (Default|CallOnAmmoEmptied self AmmoType)))
        (:then_1
          (return (LocalVariables|GetSpentAmmo) true)))
      (else
        (return 0.0 false)))
    (elif (< (LocalVariables|GetOldAmmo) 0.0)
      (Default|CallOnSpentAmmo self AmmoType (LocalVariables|GetOldAmmo) (LocalVariables|GetOldAmmo))
      (return AmmoToSpend true)
      (else
        (Default|CallOnTriedSpendEmptyAmmo self AmmoType)
        (return 0.0 false)))))