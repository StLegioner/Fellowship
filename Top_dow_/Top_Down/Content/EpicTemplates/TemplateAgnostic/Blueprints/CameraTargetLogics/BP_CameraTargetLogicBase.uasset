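; Base class for camera target logics, which each update supplies a desired location and view plane width for a camera.
; UpdateLogic interpolates the current plane width toward its target and returns it with a zero location.
; UpdateDesiredPlaneWidth changes that target by interpolating, snapping, or shifting the current value by the same delta, which preserves any blend in progress.
; Setup, Cleanup and DebugValues are empty stubs.
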(fn Setup
  (params (InOwnerActor :type Actor%20Object%20Reference) (InOwningComponent :type Actor%20Component%20Object%20Reference)))

(fn Cleanup
  (params (OwnerActor :type Actor%20Object%20Reference) (OwningComponent :type Actor%20Component%20Object%20Reference)))

(fn UpdateLogic
  (params (DeltaSeconds :type Float%20%28double-precision%29))
  (bind _output_get (Variables|Default|SetCurrentDesiredPlaneWidth (Math|Interpolation|FInterpTo (Variables|Default|GetCurrentDesiredPlaneWidth) (Variables|Default|GetTargetDesiredPlaneWidth) DeltaSeconds (Variables|Default|GetDesiredPlaneWidthInterpSpeed))))
  (return "0, 0, 0" _output_get))

(fn DebugValues
  (params (DebugLines :type Array%20of%20Debug%20Line%20Struct%20Structures) (DebugArrows :type Array%20of%20Debug%20Line%20Struct%20Structures) (DebugSpheres :type Array%20of%20Debug%20Sphere%20Struct%20Structures) (DebugStrings :type Array%20of%20Debug%20String%20Struct%20Structures))
  (return))

(fn UpdateDesiredPlaneWidth
  (params (NewDesiredPlaneWidth :type Float%20%28double-precision%29) (UpdatePlaneWidthType :type EUpdateDesiredPlaneWidthType%20Enum :default "NewEnumerator0"))
  (switch Utilities|FlowControl|Switch|SwitchonEUpdateDesiredPlaneWidthType UpdatePlaneWidthType
    (:NewEnumerator0
      (Variables|Default|SetTargetDesiredPlaneWidth NewDesiredPlaneWidth))
    (:NewEnumerator2
      (CameraTargetLogic|Protected|UpdateBaseDesiredPlaneWidthbyDelta NewDesiredPlaneWidth))
    (:NewEnumerator1
      (bind _output_get (Variables|Default|SetTargetDesiredPlaneWidth NewDesiredPlaneWidth))
      (Variables|Default|SetCurrentDesiredPlaneWidth _output_get))))

(fn UpdateBaseDesiredPlaneWidthbyDelta
  (params (NewDesiredPlaneWidth :type Float%20%28double-precision%29))
  (LocalVariables|SetBasePlaneWidthDelta (- NewDesiredPlaneWidth (Variables|Default|GetTargetDesiredPlaneWidth)))
  (Variables|Default|SetTargetDesiredPlaneWidth NewDesiredPlaneWidth)
  (Variables|Default|SetCurrentDesiredPlaneWidth (+ (Variables|Default|GetCurrentDesiredPlaneWidth) (LocalVariables|GetBasePlaneWidthDelta))))