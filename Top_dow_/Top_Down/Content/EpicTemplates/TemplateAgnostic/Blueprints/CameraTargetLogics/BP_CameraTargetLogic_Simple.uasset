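; Simple camera target logic that supplies a desired camera location and view plane width based on an owner actor.
; Setup stores the owner actor.
; Each update runs the parent logic, then leads the actor's location by its velocity scaled by a prediction multiplier.
; The view plane width is passed through from the current desired width variable, with no calculation here.
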(fn Setup
  (params (InOwnerActor :type Actor%20Object%20Reference) (InOwningComponent :type Actor%20Component%20Object%20Reference))
  (Variables|Default|SetOwner%20Actor InOwnerActor))

(fn UpdateLogic
  (params (DeltaSeconds :type Float%20%28double-precision%29))
  (bind _owner_actor (Variables|Default|GetOwner%20Actor))
  (|CallParentFunction DeltaSeconds)
  (return (+ (Transformation|GetActorLocation _owner_actor) (* (Transformation|GetVelocity _owner_actor) (Variables|Default|GetVelocityPredictionMultiplier))) (Variables|Default|GetCurrentDesiredPlaneWidth)))