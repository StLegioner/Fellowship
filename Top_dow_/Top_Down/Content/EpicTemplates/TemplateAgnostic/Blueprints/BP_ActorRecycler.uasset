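; Actor pooling manager that hands out recycled actor instances instead of spawning new ones each time.
; Requests pull an unused instance of the class, reposition it and reset it through its BP_ReusableActorComponent, or spawn one and bind its events.
; Instances move between per-class alive and unused groups on registration, reuse-ready events and destruction.
; A soft-class variant loads the class synchronously before requesting.
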(event Custom|ReusableActorDestroyed
  (params (DestroyedActor :type Actor%20Object%20Reference))
  (CallFunction|RemoveInstancefromGroup DestroyedActor (Variables|Default|GetUnusedActorGroups))
  (CallFunction|RemoveInstancefromGroup DestroyedActor (Variables|Default|GetAliveActorGroups)))

(event Custom|ActorReadyForResuse
  (params (Caller :type BP%20Reusable%20Actor%20Component%20Object%20Reference) (ActorForReuse :type Actor%20Object%20Reference))
  (CallFunction|RemoveInstancefromGroup ActorForReuse (Variables|Default|GetAliveActorGroups))
  (CallFunction|AddActortoGroup ActorForReuse (Utilities|GetClass ActorForReuse) (Variables|Default|GetUnusedActorGroups)))

(event EventRequestRegistration
  (params (ReusableActorComponent :type BP%20Reusable%20Actor%20Component%20Object%20Reference) (OwnerActor :type Actor%20Object%20Reference))
  ;[1 1 1] BPI_ActorReuseManager
  (CallFunction|AddActortoGroup OwnerActor (Utilities|GetClass OwnerActor) (select (Default|GetIsReadyforReuse ReusableActorComponent) (Variables|Default|GetUnusedActorGroups) (Variables|Default|GetAliveActorGroups))))

(fn ConstructionScript)

(fn AddActortoGroup
  (params (ActorInstance :type Actor%20Object%20Reference) (ActorClass :type Actor%20Class%20Reference) (ActorGroupArray :type Array%20of%20Actor%20Group%20Struct%20Structures))
  (for (_array_element _array_index) ActorGroupArray
    (LocalVariables|SetIdx _array_index)
    (if (== (Utilities|Struct|BreakActorGroupStruct _array_element) ActorClass)
      (Utilities|Array|AddUnique (Utilities|Struct|BreakActorGroupStruct (Utilities|Array|Get(acopy) ActorGroupArray (LocalVariables|GetIdx))) ActorInstance)
      (return)))
  (Utilities|Array|Add ActorGroupArray (Utilities|Struct|MakeActorGroupStruct ActorClass (Utilities|Array|MakeArray ActorInstance))))

(fn RemoveInstancefromGroup
  (params (ActorInstance :type Actor%20Object%20Reference) (ActorGroupArray :type Array%20of%20Actor%20Group%20Struct%20Structures))
  (LocalVariables|SetActorClass (Utilities|GetClass ActorInstance))
  (for (_array_element _array_index) ActorGroupArray
    (LocalVariables|SetIdx _array_index)
    (if (== (Utilities|Struct|BreakActorGroupStruct _array_element) (LocalVariables|GetActorClass))
      (bind _returnvalue (Utilities|Array|RemoveItem (Utilities|Struct|BreakActorGroupStruct (Utilities|Array|Get(acopy) ActorGroupArray (LocalVariables|GetIdx))) ActorInstance))
      (return _returnvalue)))
  (return false))

(fn GetInstancefromGroupandRemove
  (params (ActorClass :type Actor%20Class%20Reference) (ActorGroupArray :type Array%20of%20Actor%20Group%20Struct%20Structures))
  (for (_ _array_index) ActorGroupArray
    (LocalVariables|SetIdx _array_index)
    (if (== (Utilities|Struct|BreakActorGroupStruct (Utilities|Array|Get(acopy) ActorGroupArray (LocalVariables|GetIdx))) ActorClass)
      (if (> (Utilities|Array|Length (Utilities|Struct|BreakActorGroupStruct (Utilities|Array|Get(acopy) ActorGroupArray (LocalVariables|GetIdx)))) 0)
        (while (> (Utilities|Array|Length (Utilities|Struct|BreakActorGroupStruct (Utilities|Array|Get(acopy) ActorGroupArray (LocalVariables|GetIdx)))) 0)
          (bind _output_get (LocalVariables|SetFoundInstance (Utilities|Array|Get(acopy) (Utilities|Struct|BreakActorGroupStruct (Utilities|Array|Get(acopy) ActorGroupArray (LocalVariables|GetIdx))) (Utilities|Array|LastIndex (Utilities|Struct|BreakActorGroupStruct (Utilities|Array|Get(acopy) ActorGroupArray (LocalVariables|GetIdx)))))))
          (Utilities|FlowControl|Sequence
            (:then_0
              (Utilities|Array|RemoveIndex (Utilities|Struct|BreakActorGroupStruct (Utilities|Array|Get(acopy) ActorGroupArray (LocalVariables|GetIdx))) (Utilities|Array|LastIndex (Utilities|Struct|BreakActorGroupStruct (Utilities|Array|Get(acopy) ActorGroupArray (LocalVariables|GetIdx))))))
            (:then_1
              (Utilities|IsValid _output_get
                (:Is%20Valid
                  (return (LocalVariables|GetFoundInstance) true))))))
        (else
          (return 0 false)))))
  (return 0 false))

(fn BindtoActorEvents
  (params (Actor :type Actor%20Object%20Reference))
  (Game|BindEventtoOnDestroyed Actor (EventDispatchers|CreateEvent :!event Custom|ReusableActorDestroyed))
  (bind _output_get (LocalVariables|SetReusableActorComponent (Actor|GetComponentbyClass Actor "/Game/EpicTemplates/TemplateAgnostic/Blueprints/Components/BP_ReusableActorComponent.BP_ReusableActorComponent_C")))
  (Utilities|IsValid _output_get
    (:Is%20Valid
      (Default|BindReuseManager (LocalVariables|GetReusableActorComponent) (EventDispatchers|CreateEvent :!event Custom|ActorReadyForResuse))
      (return true))
    (:Is%20Not%20Valid
      (return false))))

(fn GetManagerActor
  (return self))

(fn RequestActorInstance
  (params (ActorClass :type Actor%20Class%20Reference) (ActorTrans :type Transform%20%28by%20ref%29) (InOwner :type Actor%20Object%20Reference) (InInstigator :type Pawn%20Object%20Reference))
  (Utilities|FlowControl|Sequence
    (:then_0
      (bind (_instance _bfoundinstance) (CallFunction|GetInstancefromGroupandRemove ActorClass (Variables|Default|GetUnusedActorGroups)))
      (if _bfoundinstance
        (bind _output_get (LocalVariables|SetTempActor _instance))
        (Transformation|SetActorTransform _output_get ActorTrans false true)
        (Actor|SetOwner (LocalVariables|GetTempActor) InOwner)
        (Variables|/Script/Engine.Actor|SetInstigator (LocalVariables|GetTempActor) InInstigator)
        (bind _output_get_2 (LocalVariables|SetReusableActorComp (Actor|GetComponentbyClass (LocalVariables|GetTempActor) "/Game/EpicTemplates/TemplateAgnostic/Blueprints/Components/BP_ReusableActorComponent.BP_ReusableActorComponent_C")))
        (Utilities|IsValid _output_get_2
          (:Is%20Valid
            (Default|ResetActor (LocalVariables|GetReusableActorComp))))
        (else
          (bind _returnvalue (Game|SpawnActorfromClass ActorClass ActorTrans "AlwaysSpawn" "MultiplyWithRoot" InOwner InInstigator))
          (bind _output_get_3 (LocalVariables|SetTempActor _returnvalue))
          (bind _actorcanbereused (CallFunction|BindtoActorEvents _output_get_3))
          (if (not _actorcanbereused)
            (return (LocalVariables|GetTempActor))))))
    (:then_1
      (CallFunction|AddActortoGroup (LocalVariables|GetTempActor) ActorClass (Variables|Default|GetAliveActorGroups))
      (return (LocalVariables|GetTempActor)))))

(fn RequestActorInstanceSoftBlocking
  (params (ActorClass :type Actor%20Soft%20Class%20Reference) (ActorTrans :type Transform%20%28by%20ref%29) (InOwner :type Actor%20Object%20Reference) (InInstigator :type Pawn%20Object%20Reference))
  (bind _returnvalue (Utilities|LoadClassAssetBlocking ActorClass))
  (bind _asactor (Utilities|Casting|CastToActorClass _returnvalue)
    (:then
      (bind _actorinstance (CallFunction|RequestActorInstance _asactor ActorTrans InOwner InInstigator))
      (return _actorinstance))
    (:CastFailed
      (return 0))))