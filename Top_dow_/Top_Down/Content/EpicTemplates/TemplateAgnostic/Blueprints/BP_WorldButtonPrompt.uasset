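; World-space button prompt actor that shows the Interact input action's button image, with optional hold-to-interact progress.
; On BeginPlay it caches the W_ButtonImage from its widget component, passes it the owning pawn's player controller and IA_Interact, and sizes it to the draw size.
; BPI_InteractPrompt events store hold mode and clamped progress, forwarding both to the widget when valid.
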(event EventBeginPlay
  (bind _widget (Variables|Default|GetWidget))
  (bind _returnvalue (Class|WidgetComponent|GetDrawSize _widget))
  ;[1 1 1] BeginPlay
  (bind _asw_button_image (Utilities|Casting|CastToW_ButtonImage (UserInterface|GetWidget (Variables|Default|GetWidget))))
  (bind _output_get (Variables|Default|SetButtonImageWidget _asw_button_image))
  (Utilities|FlowControl|Sequence
    (:then_0
      (bind _aspawn (Utilities|Casting|CastToPawn (Components|GetOwner)))
      (bind _asplayer_controller (Utilities|Casting|CastToPlayerController (Pawn|GetController _aspawn)))
      (Default|UpdateOwningPlayer (Variables|Default|GetButtonImageWidget) _asplayer_controller))
    (:then_1
      (Default|UpdateInputAction _output_get "/Game/EpicTemplates/TemplateAgnostic/Input/IA_Interact.IA_Interact")
      (Default|Resize (Variables|Default|GetButtonImageWidget) (.x _returnvalue) (.y _returnvalue)))))

(event EventUpdateHoldProgress
  (params (NewProgress :type Float%20%28double-precision%29))
  (bind _buttonimagewidget (Variables|Default|GetButtonImageWidget))
  ;[1 1 1] BPI_InteractPrompt
  (Variables|Default|SetHoldProgress (Math|Float|Clamp(Float) NewProgress))
  (Utilities|IsValid _buttonimagewidget
    (:Is%20Valid
      (Default|UpdateHoldProgress _buttonimagewidget (Variables|Default|GetHoldProgress)))))

(event EventUpdateIsHoldPrompt
  (params (bIsHoldPrompt :type Boolean))
  (bind _buttonimagewidget (Variables|Default|GetButtonImageWidget))
  ;[1 1 1] BPI_InteractPrompt
  (Variables|Default|SetIsHold bIsHoldPrompt)
  (Utilities|IsValid _buttonimagewidget
    (:Is%20Valid
      (Default|UpdateIsHoldPrompt _buttonimagewidget (Variables|Default|GetIsHold)))))

(fn ConstructionScript)