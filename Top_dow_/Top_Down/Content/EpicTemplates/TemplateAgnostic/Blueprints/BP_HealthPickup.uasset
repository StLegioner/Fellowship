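; Health pickup actor with a rotating mesh that heals an overlapping actor by a set amount, capped at max health.
; Sphere overlap searches the other actor for a BPI_HealthSource implementer, so it needs no specific character class.
; It is consumed only if health differs from max, then hides and disables collision rather than being destroyed.
; ReusableActorComponent's OnReadyForReuse event restores visibility and collision.
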(event OnReadyforReuse(ReusableActorComponent)
  (params (Caller :type BP%20Reusable%20Actor%20Component%20Object%20Reference) (ActorForReuse :type Actor%20Object%20Reference))
  (Rendering|SetActorHiddenInGame false)
  (Collision|SetActorEnableCollision true))

(event OnComponentBeginOverlap(SphereCollision)
  (params (OverlappedComponent :type Primitive%20Component%20Object%20Reference) (OtherActor :type Actor%20Object%20Reference) (OtherComp :type Primitive%20Component%20Object%20Reference) (OtherBodyIndex :type Integer) (bFromSweep :type Boolean) (SweepResult :type Hit%20Result%20Structure%20%28by%20ref%29))
  (bind _interfaceimplementingobject (CallFunction|SearchActorforInterface OtherActor "/Game/EpicTemplates/TemplateAgnostic/Blueprints/Interfaces/BPI_HealthSource.BPI_HealthSource_C" false))
  (Utilities|IsValid _interfaceimplementingobject
    (:Is%20Valid
      (bind _asbpi_health_source (Utilities|Casting|CastToBPI_HealthSource _interfaceimplementingobject))
      (bind _currenthealth (Default|GetCurrentHealth _asbpi_health_source))
      (bind _maxhealth (Default|GetMaxHealth _asbpi_health_source))
      (if (!= _currenthealth _maxhealth)
        (Default|UpdateHealth _asbpi_health_source (Math|Float|Min(Float) _maxhealth (+ _currenthealth (Variables|Default|GetHealAmount))))
        (CallFunction|DisableActor)))))

(event Custom|DisableActor
  (Rendering|SetActorHiddenInGame true)
  (Collision|SetActorEnableCollision false))

(event EventTick
  (params (DeltaSeconds :type Float%20%28single-precision%29))
  (Transformation|AddRelativeRotation (Variables|Default|GetMeshPivot) (* (Variables|Default|GetMeshRotateRate) DeltaSeconds) false true))

(fn ConstructionScript)