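; BP_DestructableHatch is a destructible hatch built on a Chaos Geometry Collection that breaks apart where it takes damage.
; HealthComponent damage events pass the hit location to ApplyHit, which uses the FieldSystem to apply a very strong radial external strain that fractures clusters, plus an outward radial velocity.
; A separate AddImpulse event pushes the Geometry Collection directly as a velocity change.
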(event OnTookDamage(HealthComponent)
  (params (Caller :type BP%20Health%20Component%20Object%20Reference) (OldHealth :type Float%20%28double-precision%29) (NewHealth :type Float%20%28double-precision%29) (SpecialDamageName :type Name :default "None") (DamageStruct :type Damage%20Struct%20Structure))
  (CallFunction|ApplyHit (.DamageLocation (Utilities|Struct|BreakDamageStruct DamageStruct))))

(event Custom|AddImpulse
  (params (Impulse :type Vector))
  (Physics|AddImpulse (Variables|Default|GetGeometryCollection) Impulse "None" true))

(event Custom|ApplyHit
  (params (HitPoint :type Vector))
  (bind _fieldsystem (Variables|Default|GetFieldSystem))
  (Class|FieldSystemComponent|ApplyPhysicsField _fieldsystem true "Field_ExternalClusterStrain" 0 (Field|SetRadialFalloff (Variables|Default|GetRadialFalloff) 999999.0 1.0 1.0 999999.0 1e+02 HitPoint "Field_FallOff_None"))
  (Class|FieldSystemComponent|ApplyPhysicsField _fieldsystem true "Field_LinearVelocity" 0 (Field|SetRadialVector (Variables|Default|GetRadialVector) 4e+02 HitPoint)))

(fn ConstructionScript)